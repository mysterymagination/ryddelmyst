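; BP_FireKeyItem is a non-equippable inventory key item that burns whoever picks it up and is used to unlock things.
; Pickup applies point fire damage to the picker.
; Use fires the Ryddelmyst character's interact ray and sends Unlock to any hit actor implementing the OpenClose interface, passing itself and returning the success result.
; Simple getters expose its display name, description and icon.
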(event `self.OnPickup`
  (params (Picker :type "Actor Object Reference"))
  (`GameplayStatics.ApplyPointDamage` Picker 10.0 (`KismetMathLibrary.MakeVector` 0.0) (`GameplayStatics.MakeHitResult` false false 0.0 0.0 (0.0 0.0 0.0) (0.0 0.0 0.0) (0.0 0.0 1.0) (0.0 0.0 1.0) null Picker) null null "/Script/Ryddelmyst.FireDamageType"))

(fn `GetDisplayDescription`
  (returns (ReturnValue :type Text))
  (return (`self.DisplayDesc`)))

(fn `GetDisplayIcon`
  (returns (ReturnValue :type "Texture2D Object Reference"))
  (return (`self.DisplayIcon`)))

(fn `GetDisplayName`
  (returns (ReturnValue :type Text))
  (return (`self.DisplayName`)))

(fn `GetEquipSlot`
  (returns (ReturnValue :type String))
  (return ""))

(fn `IsEquippable`
  (returns (ReturnValue :type Boolean))
  (return false))

(fn `OnUse`
  (params (User :type "Actor Object Reference"))
  (returns (ReturnValue :type Boolean))
  (locals (UseSuccess :type Boolean))
  (bind _asryddelmyst_character (cast `RyddelmystCharacter` User)
    (:`then`
      (bind _returnvalue (`RyddelmystCharacter.FireInteractRay` _asryddelmyst_character))
      (bind (_bblockinghit _binitialoverlap _time _distance _location _impactpoint _normal _impactnormal _physmat _hitactor) (`GameplayStatics.BreakHitResult` _returnvalue))
      (if (`KismetSystemLibrary.DoesImplementInterface` _hitactor "/Script/Ryddelmyst.OpenClose")
        (bind _returnvalue_2 (message `OpenClose.Unlock` _hitactor User self))
        (set `local.UseSuccess` _returnvalue_2)))
    (:`CastFailed`
      _))
  (return (`local.UseSuccess`)))