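; BP_LappingLavaPool is a lava pool world object that can be inspected and interacted with, with no damage logic in this graph.
; The construction script adds a static mesh and assigns it as the collision shape component.
; GenerateDescription returns a fire warning, an Observation library lore entry and an angry reaction.
; Overlap and OnInteract only print debug strings, with OnInteract also returning its InteractCapArray.
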(event `self.ReceiveActorBeginOverlap`
  (params (OtherActor :type "Actor Object Reference"))
  (`KismetSystemLibrary.PrintString` "Hello, hot stuff!"))

(fn `GenerateDescription`
  (params (BoneName :type Name))
  (returns (ReturnValue :type "Descriptor Structure"))
  (return (make `Descriptor` "Fire hot!" (make `LibraryBookData` "Lapping Lava Pool" "This lava pool sure looks deadly. Even the mighty monsters I've encountered here seem to shy away from its furnace heat!" "" "" "Observation") "ANGRY")))

(fn `OnInteract`
  (params (Interactor :type "Actor Object Reference"))
  (returns (ReturnValue :type "Array of InteractCapability Enum"))
  (`KismetSystemLibrary.PrintString` "lava interaction")
  (return (`self.InteractCapArray`)))

(fn `UserConstructionScript`
  (bind _returnvalue (`AddComponent|NODE_AddStaticMeshComponent-0`))
  (set `self.CollisionShapeComponent` _returnvalue))