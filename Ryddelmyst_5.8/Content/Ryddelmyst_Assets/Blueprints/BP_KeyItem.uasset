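; BP_KeyItem is a non-equippable inventory item that acts as a key for objects implementing the OpenClose interface.
; On use, it casts the user to RyddelmystCharacter and fires that character's interact ray.
; If the hit actor implements OpenClose, it passes itself through UnlockMessage and returns the result as the use success.
; Display name, description, icon and equip slot getters return empty values.
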(fn `GetDisplayDescription`
  (returns (ReturnValue :type Text))
  (return ""))

(fn `GetDisplayIcon`
  (returns (ReturnValue :type "Texture2D Object Reference"))
  (return null))

(fn `GetDisplayName`
  (returns (ReturnValue :type Text))
  (return ""))

(fn `GetEquipSlot`
  (returns (ReturnValue :type String))
  (return ""))

(fn `IsEquippable`
  (returns (ReturnValue :type Boolean))
  (return false))

(fn `OnUse`
  (params (User :type "Actor Object Reference"))
  (returns (ReturnValue :type Boolean))
  (locals (UseSuccess :type Boolean))
  (bind _asryddelmyst_character (cast `RyddelmystCharacter` User)
    (:`then`
      (bind _returnvalue (`RyddelmystCharacter.FireInteractRay` _asryddelmyst_character))
      (bind (_bblockinghit _binitialoverlap _time _distance _location _impactpoint _normal _impactnormal _physmat _hitactor) (`GameplayStatics.BreakHitResult` _returnvalue))
      (if (`KismetSystemLibrary.DoesImplementInterface` _hitactor "/Script/Ryddelmyst.OpenClose")
        (bind _returnvalue_2 (message `OpenClose.Unlock` _hitactor null self))
        (set `local.UseSuccess` _returnvalue_2)))
    (:`CastFailed`
      _))
  (return (`local.UseSuccess`)))