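; BP_IronSwordCloudConquestItem is an equippable Hands-slot item that grants a double jump.
; On equip, it casts the equipped actor to RyddelmystCharacter and raises its max jump count; no unequip logic here reverts it.
; Display getters return the item's name, description and icon variables, and using the item directly does nothing and returns false.
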(event `self.OnEquip`
  (params (EquippedActor :type "Actor Object Reference"))
  (bind _asryddelmyst_character (cast `RyddelmystCharacter` EquippedActor))
  (set `Character.JumpMaxCount` 2 _asryddelmyst_character))

(fn `GetDisplayDescription`
  (returns (ReturnValue :type Text))
  (return (`self.DisplayDesc`)))

(fn `GetDisplayIcon`
  (returns (ReturnValue :type "Texture2D Object Reference"))
  (return (`self.DisplayIcon`)))

(fn `GetDisplayName`
  (returns (ReturnValue :type Text))
  (return (`self.DisplayName`)))

(fn `GetEquipSlot`
  (returns (ReturnValue :type String))
  (return "Hands"))

(fn `IsEquippable`
  (returns (ReturnValue :type Boolean))
  (return true))

(fn `OnUse`
  (params (User :type "Actor Object Reference"))
  (returns (ReturnValue :type Boolean))
  (return false))