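; Reaper Treant boss that truly dies only to a "lavapool"-tagged damage source, scheduling one of two quest endings based on whether the Wood Egg was destroyed.
; Other deaths play dying, hide it, then revive it with reset stats after a timer.
; Event-manager egg danger toggles a speed boost and thorn damage on leg/body hits; egg death triggers running and updates the blackboard.
; Hit components forward collisions to HitBoxer.
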(event `self.ReceiveDestroyed`
  (if (`self.TrueDeath`)
    (`KismetSystemLibrary.PrintString` "treant destroyed upon true death flow")
    (else
      (`KismetSystemLibrary.PrintString` "treant destroyed on flow other than true death; spawning new instance "))))

(event `self.HandleDeath`
  (params (DamageCauser :type "Actor Object Reference"))
  (bind _tags (`Actor.Tags` DamageCauser))
  (bind _returnvalue (`KismetArrayLibrary.Array_Contains` _tags "lavapool"))
  ;[1 1 1] True Death
  (if (`KismetSystemLibrary.IsValid` DamageCauser)
    (for _array_element _tags
      (`KismetSystemLibrary.PrintString` (`KismetStringLibrary.Concat_StrStr` "handledeath; damage causer tag says " (`KismetStringLibrary.Conv_NameToString` _array_element) ", does it match lavapool? " (`KismetStringLibrary.Conv_BoolToString` _returnvalue) " damage causer name was " (`KismetSystemLibrary.GetDisplayName` DamageCauser))))
    (if _returnvalue
      (set `self.TrueDeath` true)
      (if (`BlackboardComponent.GetValueAsBool` (`AIController.Blackboard` (`AIBlueprintHelperLibrary.GetAIController` self)) (`self.IsWoodEggDestroyed`))
        (`KismetSystemLibrary.PrintString` "handledeath; the treant is dead via CravingQueen! 'good' end reached!")
        (set `self.QuestCompleteContext` "ending_craving_queen")
        (else
          (`KismetSystemLibrary.PrintString` "handledeath; the treant is dead via Practical Pawn! Bad end reached!")
          (set `self.QuestCompleteContext` "ending_practical_pawn")))
      (bind _asryddelmyst_game_instance (cast `RyddelmystGameInstance` (`GameplayStatics.GetGameInstance`)))
      (`GameplayStatics.PlaySoundAtLocation` "/Game/Ryddelmyst_Assets/Audio/SFX/Monsters/scream_horror.scream_horror" (`self.K2_GetActorLocation` DamageCauser) (struct) (`RyddelmystGameInstance.SFXVolumeScale` _asryddelmyst_game_instance) 1.0 0.0 null null null null)
      (bind _returnvalue_2 (`RyddelmystGameInstance.GetEventManager` _asryddelmyst_game_instance))
      (`RyddelmystEventManager.ScheduleQuestCompletionEvent` _returnvalue_2 (`GameplayStatics.GetGameInstance`) 10.0 (`self.QuestCompleteContext`))
      (`parent.HandleDeath` DamageCauser)
      (else
        (`KismetSystemLibrary.PrintString` "handledeath; false death because damage causer did not have tag lavapool")
        ;[1 1 1] False Death & Resurrection
        (bind _asbp_reaper_treant_anim (cast `/Game/Ryddelmyst_Assets/Animations/BP_ReaperTreantAnim` (`SkeletalMeshComponent.GetAnimInstance` (`self.Mesh`)) :!label _label))
        (set `/Game/Ryddelmyst_Assets/Animations/BP_ReaperTreantAnim.IsDying` true _asbp_reaper_treant_anim)
        (bind _asbp_reaper_treant_ai (cast `/Game/Ryddelmyst_Assets/Blueprints/AI/Bestiary/ReaperTreant/BP_ReaperTreantAI` (`AIBlueprintHelperLibrary.GetAIController` self)))
        (`BlackboardComponent.SetValueAsBool` (`AIController.Blackboard` _asbp_reaper_treant_ai) (`self.IsDying`) true)
        (`KismetSystemLibrary.K2_SetTimerDelegate` (delegate `Event Disappear`) 5.0)))
    (else
      (`KismetSystemLibrary.PrintString` "handledeath; false death due to invalid damage causer object")
      (goto _label))))

(event `Event Disappear`
  ;[1 1 1] False Death & Resurrection
  (`self.SetActorEnableCollision` false)
  (`self.SetActorHiddenInGame` true)
  (`KismetSystemLibrary.K2_SetTimerDelegate` (delegate `Event Revival`) 60.0))

(event `Event Revival`
  ;[1 1 1] False Death & Resurrection
  (set `/Game/Ryddelmyst_Assets/Animations/BP_ReaperTreantAnim.IsDying` false (stale `self.HandleDeath` _asbp_reaper_treant_anim))
  (set `/Game/Ryddelmyst_Assets/Animations/BP_ReaperTreantAnim.IsIdle` true (stale `self.HandleDeath` _asbp_reaper_treant_anim))
  (`BlackboardComponent.SetValueAsBool` (`AIController.Blackboard` (stale `self.HandleDeath` _asbp_reaper_treant_ai)) (`self.IsDying`) false)
  (bind _returnvalue (`BattleStatsBearer.GetStats`))
  (`BattleStats.ResetStats` _returnvalue)
  (`self.SetActorEnableCollision` true)
  (`self.SetActorHiddenInGame` false))

(event `self.ReceiveBeginPlay`
  (set `self.DeathParticleSystem` "/Game/Ryddelmyst_Assets/Particles/P_BossMonsterKillFX.P_BossMonsterKillFX")
  (`BlackboardComponent.SetValueAsVector` (`AIController.Blackboard` (`AIBlueprintHelperLibrary.GetAIController` self)) (`self.ScriptedDeathLocation`) (660.0 5400.0 210.0)))

(event `self.ReceivePossessed`
  (params (NewController :type "Controller Object Reference"))
  (`KismetSystemLibrary.K2_SetTimerDelegate` (delegate `Event Report HP`) 5.0 true)
  (bind _returnvalue (`|GenericCreateObject` "/Script/Ryddelmyst.ClawSlashAttack"))
  (set `self.Thorn Attack` _returnvalue)
  (bind _asbp_reaper_treant_ai (cast `/Game/Ryddelmyst_Assets/Blueprints/AI/Bestiary/ReaperTreant/BP_ReaperTreantAI` (`AIBlueprintHelperLibrary.GetAIController` self)))
  (set `/Game/Ryddelmyst_Assets/Blueprints/AI/Bestiary/ReaperTreant/BP_ReaperTreantAI.RightClawNerve` null _asbp_reaper_treant_ai)
  (set `/Game/Ryddelmyst_Assets/Blueprints/AI/Bestiary/ReaperTreant/BP_ReaperTreantAI.LeftClawNerve` null _asbp_reaper_treant_ai)
  (bind _asbp_reaper_treant_anim (cast `/Game/Ryddelmyst_Assets/Animations/BP_ReaperTreantAnim` (`SkeletalMeshComponent.GetAnimInstance` (`self.Mesh`)))
    (:`then`
      (set `/Game/Ryddelmyst_Assets/Animations/BP_ReaperTreantAnim.ReaperTreantAI` _asbp_reaper_treant_ai _asbp_reaper_treant_anim)
      (bind _asryddelmyst_game_instance (cast `RyddelmystGameInstance` (`GameplayStatics.GetGameInstance`)))
      (bind _returnvalue_2 (`RyddelmystGameInstance.GetEventManager` _asryddelmyst_game_instance))
      (add `RyddelmystEventManager.WoodEggDeathEvent` _returnvalue_2 (delegate `OnWoodEggDeath`))
      (add `RyddelmystEventManager.WoodEggDangerEvent` _returnvalue_2 (delegate `OnWoodEggDanger`)))
    (:`CastFailed`
      (`KismetSystemLibrary.PrintString` "failed to cast anim from treant skel to treantanim"))))

(event `OnWoodEggDanger`
  (params (InDanger :type Boolean))
  (bind _extremitycapsulerightleg (`self.ExtremityCapsuleRightLeg`))
  (bind _returnvalue (`BattleStatsBearer.GetStats`))
  (if InDanger
    (add `PrimitiveComponent.OnComponentHit` _extremitycapsulerightleg (delegate `Thorn Mode Activated`))
    (add `PrimitiveComponent.OnComponentHit` (`self.ExtremityCapsuleLeftLeg`) (delegate `Thorn Mode Activated`))
    (add `PrimitiveComponent.OnComponentHit` (`self.BodyBox`) (delegate `Thorn Mode Activated`))
    (bind _statsmap (break `BattleStatsData` (`BattleStats.StatsData` _returnvalue)))
    (bind _value (`BlueprintMapLibrary.Map_Find` _statsmap "Speed"))
    (`BlueprintMapLibrary.Map_Add` _statsmap "Speed" (* _value (`self.PanicSpeedMod`)))
    (else
      (remove `PrimitiveComponent.OnComponentHit` _extremitycapsulerightleg (delegate `Thorn Mode Activated`))
      (remove `PrimitiveComponent.OnComponentHit` (`self.ExtremityCapsuleLeftLeg`) (delegate `Thorn Mode Activated`))
      (remove `PrimitiveComponent.OnComponentHit` (`self.BodyBox`) (delegate `Thorn Mode Activated`))
      (`BlueprintMapLibrary.Map_Add` _statsmap "Speed" (/ _value (`self.PanicSpeedMod`)))))
  (`BattleStatsBearer.HandleStatModification` "Speed"))

(event `Thorn Mode Activated`
  (params (HitComponent :type "PrimitiveComponent Object Reference") (OtherActor :type "Actor Object Reference") (OtherComp :type "PrimitiveComponent Object Reference") (NormalImpulse :type "Vector Structure") (Hit :type "HitResult Structure (by ref)"))
  (`Attack.OnHit` (`self.Thorn Attack`) (`BattleStats.StatsData` (stale `OnWoodEggDanger` _returnvalue)) HitComponent OtherActor OtherComp NormalImpulse Hit)
  (`KismetSystemLibrary.PrintString` "thorn attack delivered"))

(event `OnWoodEggDeath`
  (params (DeathLocation :type "Vector Structure"))
  (bind _blackboard (`AIController.Blackboard` (`AIBlueprintHelperLibrary.GetAIController` self)))
  (`KismetSystemLibrary.PrintString` "the wood egg has been destroyed!")
  (`self.Run`)
  (`BlackboardComponent.SetValueAsVector` _blackboard (`self.LastLocationOfWoodEgg`) DeathLocation)
  (`BlackboardComponent.SetValueAsBool` _blackboard (`self.IsWoodEggDestroyed`) true))

(event `Event Report HP`
  (bind _returnvalue (`BattleStatsBearer.GetStats`))
  (`KismetSystemLibrary.PrintString` (`KismetStringLibrary.Concat_StrStr` "Treant HP is " (`KismetStringLibrary.Conv_DoubleToString` (`BlueprintMapLibrary.Map_Find` (`.StatsMap` (break `BattleStatsData` (`BattleStats.StatsData` _returnvalue))) "HP")))))

(event `self.BodyBox.OnComponentHit`
  (params (HitComponent :type "PrimitiveComponent Object Reference") (OtherActor :type "Actor Object Reference") (OtherComp :type "PrimitiveComponent Object Reference") (NormalImpulse :type "Vector Structure") (Hit :type "HitResult Structure (by ref)"))
  (`HitBoxerComponent.OnHit` (`self.HitBoxer`) HitComponent OtherActor OtherComp NormalImpulse Hit))

(event `self.HeadBox.OnComponentHit`
  (params (HitComponent :type "PrimitiveComponent Object Reference") (OtherActor :type "Actor Object Reference") (OtherComp :type "PrimitiveComponent Object Reference") (NormalImpulse :type "Vector Structure") (Hit :type "HitResult Structure (by ref)"))
  (`HitBoxerComponent.OnHit` (`self.HitBoxer`) HitComponent OtherActor OtherComp NormalImpulse Hit))

(event `self.ExtremityCapsuleRightLeg.OnComponentHit`
  (params (HitComponent :type "PrimitiveComponent Object Reference") (OtherActor :type "Actor Object Reference") (OtherComp :type "PrimitiveComponent Object Reference") (NormalImpulse :type "Vector Structure") (Hit :type "HitResult Structure (by ref)"))
  (`HitBoxerComponent.OnHit` (`self.HitBoxer`) HitComponent OtherActor OtherComp NormalImpulse Hit))

(event `self.ExtremityCapsuleLeftLeg.OnComponentHit`
  (params (HitComponent :type "PrimitiveComponent Object Reference") (OtherActor :type "Actor Object Reference") (OtherComp :type "PrimitiveComponent Object Reference") (NormalImpulse :type "Vector Structure") (Hit :type "HitResult Structure (by ref)"))
  (`HitBoxerComponent.OnHit` (`self.HitBoxer`) HitComponent OtherActor OtherComp NormalImpulse Hit))

(event `self.ClawCapsuleLeft.OnComponentHit`
  (params (HitComponent :type "PrimitiveComponent Object Reference") (OtherActor :type "Actor Object Reference") (OtherComp :type "PrimitiveComponent Object Reference") (NormalImpulse :type "Vector Structure") (Hit :type "HitResult Structure (by ref)"))
  (`KismetSystemLibrary.PrintString` "shapely left claw hit")
  (`HitBoxerComponent.OnHit` (`self.HitBoxer`) HitComponent OtherActor OtherComp NormalImpulse Hit))

(event `self.ClawCapsuleRight.OnComponentHit`
  (params (HitComponent :type "PrimitiveComponent Object Reference") (OtherActor :type "Actor Object Reference") (OtherComp :type "PrimitiveComponent Object Reference") (NormalImpulse :type "Vector Structure") (Hit :type "HitResult Structure (by ref)"))
  (`KismetSystemLibrary.PrintString` "shapely right claw hit")
  (`HitBoxerComponent.OnHit` (`self.HitBoxer`) HitComponent OtherActor OtherComp NormalImpulse Hit))

(event `self.ExtremityCapsuleLeftArm.OnComponentHit`
  (params (HitComponent :type "PrimitiveComponent Object Reference") (OtherActor :type "Actor Object Reference") (OtherComp :type "PrimitiveComponent Object Reference") (NormalImpulse :type "Vector Structure") (Hit :type "HitResult Structure (by ref)"))
  (`HitBoxerComponent.OnHit` (`self.HitBoxer`) HitComponent OtherActor OtherComp NormalImpulse Hit))

(event `self.ExtremityCapsuleRightArm.OnComponentHit`
  (params (HitComponent :type "PrimitiveComponent Object Reference") (OtherActor :type "Actor Object Reference") (OtherComp :type "PrimitiveComponent Object Reference") (NormalImpulse :type "Vector Structure") (Hit :type "HitResult Structure (by ref)"))
  (`HitBoxerComponent.OnHit` (`self.HitBoxer`) HitComponent OtherActor OtherComp NormalImpulse Hit))

(fn `Thorn Mode`
  (params (Activate :type Boolean))
  (if Activate
    _))

(fn `UserConstructionScript`)