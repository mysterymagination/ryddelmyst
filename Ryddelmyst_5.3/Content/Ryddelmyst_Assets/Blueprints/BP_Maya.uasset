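; BP_Maya is the Maya Blueprint, an interactable that can be described.
; GetBody exposes its capsule hitbox, and OnInteract returns its InteractCaps regardless of the interactor.
; GenerateDescription fills SelfDesc with a random line from the Desc array and an independently rolled random reaction, so text and mood are unpaired.
; The event graph and construction script hold no logic.
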(event `self.ReceiveBeginPlay`)

(fn `GenerateDescription`
  (returns (ReturnValue :type "Descriptor Structure"))
  (locals (Reaction :type "InteractReactions Enum") (SelfDesc :type "Descriptor Structure"))
  (bind _desc (`self.Desc`))
  (switch `int` (`KismetMathLibrary.RandomIntegerInRange` 0 4)
    (:`0`
      (set `local.Reaction` "HAPPY"))
    (:`1`
      (set `local.Reaction` "FLIRTY"))
    (:`2`
      (set `local.Reaction` "EMBARRASSED"))
    (:`3`
      (set `local.Reaction` "CONFUSED"))
    (:`4`
      (set `local.Reaction` "ELDRITCH")))
  (bind _structout (setmembers `Descriptor` :`StructRef` (`local.SelfDesc`) :`LocalizedDescription` (`KismetTextLibrary.Conv_StringToText` (`|GetArrayItem` _desc (`KismetMathLibrary.RandomIntegerInRange` 0 (- (`KismetArrayLibrary.Array_Length` _desc) 1)))) :`Reaction` (`local.Reaction`)))
  (return _structout))

(fn `GetBody`
  (returns (ReturnValue :type "BodyCapsuleComponent Object Reference"))
  (return (`self.BodyCapsuleHitBox`)))

(fn `OnInteract`
  (params (Interactor :type "Actor Object Reference"))
  (returns (ReturnValue :type "Array of InteractCapability Enum"))
  (return (`self.InteractCaps`)))

(fn `UserConstructionScript`)