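; BP_MollyStatue is an interactable statue that supplies a look description with a confused reaction.
; GenerateDescription packs the description and reaction into a descriptor, swapping in placeholder text on every look after the first via the IsFirstLook flag.
; OnInteract only prints the current description and returns its interact capability array.
; The event graph and construction script are empty.
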(fn `GenerateDescription`
  (returns (ReturnValue :type "Descriptor Structure"))
  (if (not (`self.IsFirstLook`))
    (set `self.Description` "sdf"))
  (bind _structout (setmembers `Descriptor` :`StructRef` (`self.Descriptor`) :`LocalizedDescription` (`self.Description`) :`Reaction` "CONFUSED"))
  (set `self.IsFirstLook` false)
  (return _structout))

(fn `OnInteract`
  (params (Interactor :type "Actor Object Reference"))
  (returns (ReturnValue :type "Array of InteractCapability Enum"))
  (`KismetSystemLibrary.PrintString` (`KismetTextLibrary.Conv_TextToString` (`self.Description`)))
  (return (`self.InteractCapArray`)))

(fn `UserConstructionScript`)