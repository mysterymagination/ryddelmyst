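; BP_RainbowShardItem is a non-equippable usable item that restores a Ryddelmyst character's health and magic.
; On use, it casts the user to RyddelmystCharacter, passes that character's max health and max magic to UpdateHealth and UpdateMagic, then reports success.
; Simple getters supply its display name, description and icon, while the equip slot is left empty.
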(fn `GetDisplayDescription`
  (returns (ReturnValue :type Text))
  (return (`self.DisplayDesc`)))

(fn `GetDisplayIcon`
  (returns (ReturnValue :type "Texture2D Object Reference"))
  (return (`self.DisplayIcon`)))

(fn `GetDisplayName`
  (returns (ReturnValue :type Text))
  (return (`self.DisplayName`)))

(fn `GetEquipSlot`
  (returns (ReturnValue :type String))
  (return ""))

(fn `IsEquippable`
  (returns (ReturnValue :type Boolean))
  (return false))

(fn `OnUse`
  (params (User :type "Actor Object Reference"))
  (returns (ReturnValue :type Boolean))
  (bind _asryddelmyst_character (cast `RyddelmystCharacter` User))
  (`RyddelmystCharacter.UpdateHealth` _asryddelmyst_character (`RyddelmystCharacter.GetMaxHealth` _asryddelmyst_character))
  (`RyddelmystCharacter.UpdateMagic` _asryddelmyst_character (`RyddelmystCharacter.GetMaxMagic` _asryddelmyst_character))
  (return true))