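; BP_Treasurechest is an interactable chest that plays lid animations and gives its treasure to the opening RyddelmystCharacter once.
; Open either reports the lock or constructs the Treasure class, clears it, and adds it as equipment or inventory.
; Unlock accepts only the Key class, while Lock always fails.
; HUD dialogue reports outcomes, with Maya portraits reacting to locked, treasure or empty results; OnInteract returns the chest's interaction capabilities.
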(event `self.Open`
  (params (Opener :type "Actor Object Reference"))
  (bind _treasure (`self.Treasure`))
  (bind _asryddelmyst_character (cast `RyddelmystCharacter` Opener))
  (if (`self.Locked`)
    (bind _hud (`RyddelmystCharacter.HUD` _asryddelmyst_character))
    (`RyddelmystHUD.ShowDialogue` _hud "/Game/Ryddelmyst_Assets/Textures/maya_portraits_Sprite_Angry.maya_portraits_Sprite_Angry" (`KismetTextLibrary.Conv_StringToText` (`KismetStringLibrary.Concat_StrStr` (`KismetSystemLibrary.GetObjectName` self) " is locked tight!")))
    (else
      (`SkeletalMeshComponent.PlayAnimation` (`self.SkeletalMesh`) "/Game/Ryddelmyst_Assets/Meshes/SK_Treasurechest_Anim_Treasure_Open_Lid.SK_Treasurechest_Anim_Treasure_Open_Lid" false)
      (set `self.Opened` true)
      (if (`KismetSystemLibrary.IsValidClass` _treasure)
        (bind _returnvalue (`|GenericCreateObject` _asryddelmyst_character _treasure))
        (bind _returnvalue_2 (message `Item.GetDisplayDescription` _returnvalue))
        (set `self.Treasure` null)
        (bind _returnvalue_3 (message `Item.IsEquippable` _returnvalue))
        (if _returnvalue_3
          (`RyddelmystCharacter.AddEquippedItem` _asryddelmyst_character _returnvalue)
          (else
            (`RyddelmystCharacter.AddInventoryItem` _asryddelmyst_character _returnvalue)))
        ;[1 1 1] TODO: ideally we'd have the treasure itself be describable so we can have a rewaction based on that, but happy is good enough for now.
        (`RyddelmystHUD.ShowDialogue` _hud "/Game/Ryddelmyst_Assets/Textures/maya_portraits_Sprite_Happy.maya_portraits_Sprite_Happy" _returnvalue_2)
        (else
          (`RyddelmystHUD.ShowDialogue` _hud "/Game/Ryddelmyst_Assets/Textures/maya_portraits_Sprite_Weary.maya_portraits_Sprite_Weary" "There's nothing inside; what rotten luck!"))))))

(event `self.Close`
  (params (Closer :type "Actor Object Reference"))
  (`SkeletalMeshComponent.PlayAnimation` (`self.SkeletalMesh`) "/Game/Ryddelmyst_Assets/Meshes/SK_Treasurechest_Anim_Treasure_Close_Lid.SK_Treasurechest_Anim_Treasure_Close_Lid" false)
  (set `self.Opened` false))

(fn `IsOpen`
  (returns (ReturnValue :type Boolean))
  (return (`self.Opened`)))

(fn `Lock`
  (params (Locker :type "Actor Object Reference") (Item :type "Object Object Reference"))
  (returns (ReturnValue :type Boolean))
  (return false))

(fn `OnInteract`
  (params (Interactor :type "Actor Object Reference"))
  (returns (ReturnValue :type "Array of InteractCapability Enum"))
  (return (`self.InteractCapArray`)))

(fn `Unlock`
  (params (Unlocker :type "Actor Object Reference") (Item :type "Object Object Reference"))
  (returns (ReturnValue :type Boolean))
  (locals (ResultString :type String) (ResultText :type Text) (UnlockSuccess :type Boolean))
  (bind _returnvalue (`KismetSystemLibrary.GetObjectName` self))
  (bind _returnvalue_2 (message `Item.GetDisplayName` Item))
  (if (== (`GameplayStatics.GetObjectClass` Item) (`self.Key`))
    (set `self.Locked` false)
    (set `local.UnlockSuccess` true)
    (set `local.ResultText` (`KismetTextLibrary.Conv_StringToText` (`KismetStringLibrary.Concat_StrStr` _returnvalue " unlocks with a satisfying but mildly concerning *clonk*!")))
    (else
      (set `local.UnlockSuccess` false)
      (if (`self.Locked`)
        (bind _returnvalue_3 (`KismetStringLibrary.Concat_StrStr` (`KismetStringLibrary.Concat_StrStr` (`KismetTextLibrary.Conv_TextToString` _returnvalue_2) " doesn't fit in ") _returnvalue))
        (bind _output_get (set `local.ResultString` (`KismetStringLibrary.Concat_StrStr` _returnvalue_3 ", which is still locked")))
        (set `local.ResultText` (`KismetTextLibrary.Conv_StringToText` _output_get))
        (else
          (bind _output_get_2 (set `local.ResultString` (`KismetStringLibrary.Concat_StrStr` _returnvalue_3 ", whish is already open btw")))
          (set `local.ResultText` (`KismetTextLibrary.Conv_StringToText` _output_get_2))))))
  (bind _asryddelmyst_hud (cast `RyddelmystHUD` (`PlayerController.GetHUD` (`GameplayStatics.GetPlayerController` 0))))
  (`RyddelmystHUD.ShowDialogue` _asryddelmyst_hud null (`local.ResultText`))
  (return (`local.UnlockSuccess`)))

(fn `UserConstructionScript`)