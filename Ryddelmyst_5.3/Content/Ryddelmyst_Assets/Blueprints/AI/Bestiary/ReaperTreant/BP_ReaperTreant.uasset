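; Reaper Treant enemy character that dies, disappears and later revives in place.
; HandleDeath flags dying on the AnimBP and AI blackboard, then chained timers hide the actor without collision and later restore it with reset stats.
; Hit events from body, head, limb and claw shapes all forward to HitBoxer.
; Possession starts a looping debug HP printout; an unconnected chain for linking claw nerves and AnimBP to the AI controller never runs.
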(event `Event Disappear`
  ;[1 1 1] Death & Resurrection
  (`self.SetActorEnableCollision` false)
  (`self.SetActorHiddenInGame` true)
  (`KismetSystemLibrary.K2_SetTimerDelegate` (delegate `Event Revival`) 60.0))

(event `self.HandleDeath`
  ;[1 1 1] Death & Resurrection
  (bind _asbp_reaper_treant_anim (cast `/Game/Ryddelmyst_Assets/Animations/BP_ReaperTreantAnim` (`SkeletalMeshComponent.GetAnimInstance` (`self.Mesh`))))
  (set `/Game/Ryddelmyst_Assets/Animations/BP_ReaperTreantAnim.IsDying` true _asbp_reaper_treant_anim)
  (bind _asbp_reaper_treant_ai (cast `/Game/Ryddelmyst_Assets/Blueprints/AI/Bestiary/ReaperTreant/BP_ReaperTreantAI` (`AIBlueprintHelperLibrary.GetAIController` self)))
  (`BlackboardComponent.SetValueAsBool` (`AIController.Blackboard` _asbp_reaper_treant_ai) (`self.IsDying`) true)
  (`KismetSystemLibrary.K2_SetTimerDelegate` (delegate `Event Disappear`) 5.0))

(event `Event Revival`
  ;[1 1 1] Death & Resurrection
  (set `/Game/Ryddelmyst_Assets/Animations/BP_ReaperTreantAnim.IsDying` false (stale `self.HandleDeath` _asbp_reaper_treant_anim))
  (set `/Game/Ryddelmyst_Assets/Animations/BP_ReaperTreantAnim.IsIdle` true (stale `self.HandleDeath` _asbp_reaper_treant_anim))
  (`BlackboardComponent.SetValueAsBool` (`AIController.Blackboard` (stale `self.HandleDeath` _asbp_reaper_treant_ai)) (`self.IsDying`) false)
  (bind _returnvalue (`BattleStatsBearer.GetStats`))
  (`BattleStats.ResetStats` _returnvalue)
  (`self.SetActorEnableCollision` true)
  (`self.SetActorHiddenInGame` false))

(event `self.ReceivePossessed`
  (params (NewController :type "Controller Object Reference"))
  (`KismetSystemLibrary.K2_SetTimerDelegate` (delegate `Event Report HP`) 5.0 true))

(event `Event Report HP`
  (bind _returnvalue (`BattleStatsBearer.GetStats`))
  (`KismetSystemLibrary.PrintString` (`KismetStringLibrary.Concat_StrStr` "Treant HP is " (`KismetStringLibrary.Conv_DoubleToString` (`BlueprintMapLibrary.Map_Find` (`.StatsMap` (break `BattleStatsData` (`BattleStats.StatsData` _returnvalue))) "HP")))))

(event `self.BodyBox.OnComponentHit`
  (params (HitComponent :type "PrimitiveComponent Object Reference") (OtherActor :type "Actor Object Reference") (OtherComp :type "PrimitiveComponent Object Reference") (NormalImpulse :type "Vector Structure") (Hit :type "HitResult Structure (by ref)"))
  (`HitBoxerComponent.OnHit` (`self.HitBoxer`) HitComponent OtherActor OtherComp NormalImpulse Hit))

(event `self.HeadBox.OnComponentHit`
  (params (HitComponent :type "PrimitiveComponent Object Reference") (OtherActor :type "Actor Object Reference") (OtherComp :type "PrimitiveComponent Object Reference") (NormalImpulse :type "Vector Structure") (Hit :type "HitResult Structure (by ref)"))
  (`HitBoxerComponent.OnHit` (`self.HitBoxer`) HitComponent OtherActor OtherComp NormalImpulse Hit))

(event `self.ExtremityCapsuleRightLeg.OnComponentHit`
  (params (HitComponent :type "PrimitiveComponent Object Reference") (OtherActor :type "Actor Object Reference") (OtherComp :type "PrimitiveComponent Object Reference") (NormalImpulse :type "Vector Structure") (Hit :type "HitResult Structure (by ref)"))
  (`HitBoxerComponent.OnHit` (`self.HitBoxer`) HitComponent OtherActor OtherComp NormalImpulse Hit))

(event `self.ExtremityCapsuleLeftLeg.OnComponentHit`
  (params (HitComponent :type "PrimitiveComponent Object Reference") (OtherActor :type "Actor Object Reference") (OtherComp :type "PrimitiveComponent Object Reference") (NormalImpulse :type "Vector Structure") (Hit :type "HitResult Structure (by ref)"))
  (`HitBoxerComponent.OnHit` (`self.HitBoxer`) HitComponent OtherActor OtherComp NormalImpulse Hit))

(event `self.ClawCapsuleLeft.OnComponentHit`
  (params (HitComponent :type "PrimitiveComponent Object Reference") (OtherActor :type "Actor Object Reference") (OtherComp :type "PrimitiveComponent Object Reference") (NormalImpulse :type "Vector Structure") (Hit :type "HitResult Structure (by ref)"))
  (`KismetSystemLibrary.PrintString` "shapely left claw hit")
  (`HitBoxerComponent.OnHit` (`self.HitBoxer`) HitComponent OtherActor OtherComp NormalImpulse Hit))

(event `self.ClawCapsuleRight.OnComponentHit`
  (params (HitComponent :type "PrimitiveComponent Object Reference") (OtherActor :type "Actor Object Reference") (OtherComp :type "PrimitiveComponent Object Reference") (NormalImpulse :type "Vector Structure") (Hit :type "HitResult Structure (by ref)"))
  (`KismetSystemLibrary.PrintString` "shapely right claw hit")
  (`HitBoxerComponent.OnHit` (`self.HitBoxer`) HitComponent OtherActor OtherComp NormalImpulse Hit))

(event `self.ExtremityCapsuleLeftArm.OnComponentHit`
  (params (HitComponent :type "PrimitiveComponent Object Reference") (OtherActor :type "Actor Object Reference") (OtherComp :type "PrimitiveComponent Object Reference") (NormalImpulse :type "Vector Structure") (Hit :type "HitResult Structure (by ref)"))
  (`HitBoxerComponent.OnHit` (`self.HitBoxer`) HitComponent OtherActor OtherComp NormalImpulse Hit))

(event `self.ExtremityCapsuleRightArm.OnComponentHit`
  (params (HitComponent :type "PrimitiveComponent Object Reference") (OtherActor :type "Actor Object Reference") (OtherComp :type "PrimitiveComponent Object Reference") (NormalImpulse :type "Vector Structure") (Hit :type "HitResult Structure (by ref)"))
  (`HitBoxerComponent.OnHit` (`self.HitBoxer`) HitComponent OtherActor OtherComp NormalImpulse Hit))

(fn `UserConstructionScript`)