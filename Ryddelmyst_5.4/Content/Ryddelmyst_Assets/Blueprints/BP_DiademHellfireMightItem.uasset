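; BP_DiademHellfireMightItem is an item Blueprint for a Hellfire Might diadem that equips in the Head slot.
; It reports itself as equippable, and its OnUse does nothing but return false.
; Display icon, name and description getters return the asset's own variables.
; The graphs shown contain no stat or effect logic.
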(fn `GetDisplayDescription`
  (returns (ReturnValue :type Text))
  (return (`self.DisplayDesc`)))

(fn `GetDisplayIcon`
  (returns (ReturnValue :type "Texture2D Object Reference"))
  (return (`self.DisplayIcon`)))

(fn `GetDisplayName`
  (returns (ReturnValue :type Text))
  (return (`self.DisplayName`)))

(fn `GetEquipSlot`
  (returns (ReturnValue :type String))
  (return "Head"))

(fn `IsEquippable`
  (returns (ReturnValue :type Boolean))
  (return true))

(fn `OnUse`
  (params (User :type "Actor Object Reference"))
  (returns (ReturnValue :type Boolean))
  (return false))