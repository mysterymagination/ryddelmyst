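; Character Blueprint for Maya, with a jump sound, a body hitbox getter and interaction hooks.
; Receives exported particle data and tests each position against the actor's bounds to detect woodfire breath.
; On a hit, it constructs a WoodfirebreathAttack on the nearest BP_VerdantGolem, assumed to be the attacker, and calls OnHit against Maya's capsule.
; Interaction returns InteractCaps, while descriptions pair random text with a random reaction.
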(event `self.ReceiveBeginPlay`)

(event `InputAction|Jump`
  (params (Key :type "Key Structure"))
  (:`Released`
    (`GameplayStatics.PlaySoundAtLocation` "/Game/Ryddelmyst_Assets/Audio/SFX/bfxr_sounds/Jump.Jump" (`self.K2_GetActorLocation`) (struct) 0.5 1.0 0.0 null null null null)))

(event `self.ReceiveParticleData`
  (params (Data :type "Array of BasicParticleData Structure (by ref)") (NiagaraSystem :type "NiagaraSystem Object Reference") (SimulationPositionOffset :type "Vector Structure (by ref)"))
  (bind (_origin _boxextent) (`self.GetActorBounds` true))
  (for _array_element Data
    (if (`KismetMathLibrary.IsPointInBox` (`.Position` (break `BasicParticleData` _array_element)) _origin _boxextent)
      (`KismetSystemLibrary.PrintString` "oh god fire!!!")
      (bind _outactors (`GameplayStatics.GetAllActorsOfClass` "/Game/Ryddelmyst_Assets/Blueprints/AI/Bestiary/VerdantGolem/BP_VerdantGolem.BP_VerdantGolem_C"))
      (bind (_distance _returnvalue) (`GameplayStatics.FindNearestActor` (`self.K2_GetActorLocation`) _outactors))
      (bind _returnvalue_2 (`|GenericCreateObject` _returnvalue "/Script/Ryddelmyst.WoodfirebreathAttack"))
      (bind _asmonster (cast `Monster` _returnvalue))
      (bind _asbp_verdant_golem (cast `/Game/Ryddelmyst_Assets/Blueprints/AI/Bestiary/VerdantGolem/BP_VerdantGolem` _asmonster))
      (`Attack.OnHit` _returnvalue_2 (`BattleStats.StatsData` (`Monster.MonsterStats` _asmonster)) (`/Game/Ryddelmyst_Assets/Blueprints/AI/Bestiary/VerdantGolem/BP_VerdantGolem.BodyBox` _asbp_verdant_golem) self (`self.BodyCapsuleHitBox`) (0.0 0.0 0.0) (`GameplayStatics.MakeHitResult` false))
      (else
        (`KismetSystemLibrary.PrintString` "woodfirebreath collided with something, but not maya")))))

(fn `GenerateDescription`
  (returns (ReturnValue :type "Descriptor Structure"))
  (locals (Reaction :type "InteractReactions Enum") (SelfDesc :type "Descriptor Structure"))
  (bind _desc (`self.Desc`))
  (switch `int` (`KismetMathLibrary.RandomIntegerInRange` 0 4)
    (:`0`
      (set `local.Reaction` "HAPPY"))
    (:`1`
      (set `local.Reaction` "FLIRTY"))
    (:`2`
      (set `local.Reaction` "EMBARRASSED"))
    (:`3`
      (set `local.Reaction` "CONFUSED"))
    (:`4`
      (set `local.Reaction` "ELDRITCH")))
  (bind _structout (setmembers `Descriptor` :`StructRef` (`local.SelfDesc`) :`LocalizedDescription` (`KismetTextLibrary.Conv_StringToText` (`|GetArrayItem` _desc (`KismetMathLibrary.RandomIntegerInRange` 0 (- (`KismetArrayLibrary.Array_Length` _desc) 1)))) :`Reaction` (`local.Reaction`)))
  (return _structout))

(fn `GetBody`
  (returns (ReturnValue :type "BodyCapsuleComponent Object Reference"))
  (return (`self.BodyCapsuleHitBox`)))

(fn `OnInteract`
  (params (Interactor :type "Actor Object Reference"))
  (returns (ReturnValue :type "Array of InteractCapability Enum"))
  (return (`self.InteractCaps`)))

(fn `UserConstructionScript`)