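; Interactable Yvyteph Mastermind character that the player can examine for descriptions and a lore entry.
; GenerateDescription picks text and reaction by bone name, with a general fallback, and attaches the same Observation lore to every result.
; It also plays a cackle at the actor's location, scaled by the game instance's SFX volume.
; OnInteract swaps the DESCRIBABLE capability for LOREABLE and returns the capability array.
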(fn `GenerateDescription`
  (params (BoneName :type Name))
  (returns (ReturnValue :type "Descriptor Structure"))
  (bind _librarybookdata (make `LibraryBookData` "Yvyteph Mastermind" "She's been pulling the strings all along! Well, it was fairly obvious I suppose, but still. Rude! Anyway, it certainly seems like I will need to play by her rules in this game... assuming I play at all. Also cheating is the gift man gives himself, so maybe I can play to win after all." "" "" "Observation"))
  (switch `name` BoneName
    (:`Default`
      (set `self.Desc` (make `Descriptor` (`self.GeneralDesc`) _librarybookdata "ANGRY")))
    (:`Face`
      (set `self.Desc` (make `Descriptor` (`self.FaceDesc`) _librarybookdata "SAD")))
    (:`Boobs`
      (set `self.Desc` (make `Descriptor` (`self.BoobsDesc`) _librarybookdata "CONFUSED")))
    (:`Lady Garden`
      (set `self.Desc` (make `Descriptor` (`self.LadyGardenDesc`) _librarybookdata "ELDRITCH"))))
  (bind _asryddelmyst_game_instance (cast `RyddelmystGameInstance` (`GameplayStatics.GetGameInstance`))
    (:`then`
      (`GameplayStatics.PlaySoundAtLocation` "/Game/Ryddelmyst_Assets/Audio/VO/Maya/ghostly_cackle_laugh_1.ghostly_cackle_laugh_1" (`self.K2_GetActorLocation`) (struct) (`RyddelmystGameInstance.SFXVolumeScale` _asryddelmyst_game_instance) 1.0 0.0 null null null null))
    (:`CastFailed`
      _))
  (return (`self.Desc`)))

(fn `OnInteract`
  (params (Interactor :type "Actor Object Reference"))
  (returns (ReturnValue :type "Array of InteractCapability Enum"))
  (bind _interactcaparray (`self.InteractCapArray`))
  (`KismetArrayLibrary.Array_RemoveItem` _interactcaparray "DESCRIBABLE")
  (`KismetArrayLibrary.Array_Add` _interactcaparray "LOREABLE")
  (return _interactcaparray))

(fn `UserConstructionScript`
  (`parent.UserConstructionScript`))