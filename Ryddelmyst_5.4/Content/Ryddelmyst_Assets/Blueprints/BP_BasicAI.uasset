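; BP_BasicAI is a bare-bones AI controller that repeatedly sends its controlled pawn to one hardcoded world location.
; BeginPlay starts a looping timer that calls the Move event by name every few seconds.
; Move issues an AI MoveTo, then prints the pawn, movement result and destination as debug output from the immediate exec pin, without handling success or failure.
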(event `self.ReceiveTick`
  (params (DeltaSeconds :type "Float (single-precision)")))

(event `self.ReceiveBeginPlay`
  (`KismetSystemLibrary.K2_SetTimer` null "Move" 5.0 true))

(event `Move`
  (bind _returnvalue (`KismetMathLibrary.MakeVector` -740.0 -530.0 350.0))
  (bind _returnvalue_2 (`self.K2_GetPawn`))
  (bind _movementresult (`|AIMoveTo` _returnvalue_2 _returnvalue null)
    (:`then`
      (`KismetSystemLibrary.PrintString` (`KismetStringLibrary.Concat_StrStr` "controlled pawn is: " (`KismetStringLibrary.Conv_ObjectToString` _returnvalue_2)))
      (`KismetSystemLibrary.PrintString` (`KismetStringLibrary.Concat_StrStr` "moving resulted in: " (`|GetEnumeratorNameAsString` _movementresult)))
      (`KismetSystemLibrary.PrintString` (`KismetStringLibrary.Concat_StrStr` "ai moving to: " (`KismetStringLibrary.Conv_VectorToString` _returnvalue))))))

(fn `UserConstructionScript`)