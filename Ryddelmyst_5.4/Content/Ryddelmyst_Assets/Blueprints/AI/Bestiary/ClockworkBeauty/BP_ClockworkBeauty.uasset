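; Clockwork Beauty enemy pawn in the bestiary, with blaster bolt, bullet spray and judgement ray attacks plus randomized interaction descriptions.
; The blaster spawns a bolt ahead of the pawn, passes its stats into the weapon message, and clears a blackboard charge flag until a cooldown timer restores it.
; The spray builds debug-drawn spline guides that launch flame bullets.
; The judgement ray only prints, and BeginPlay enables spline display.
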(event `self.ReceiveBeginPlay`
  (`KismetSystemLibrary.PrintString` "showing splines")
  (`KismetSystemLibrary.ExecuteConsoleCommand` "show splines" null))

(event `BlasterBoltFired`
  (`KismetSystemLibrary.K2_SetTimerDelegate` (delegate `BlasterBoltRecharge`) (`self.BlasterCoolDown`)))

(event `BlasterBoltRecharge`
  (bind _asbp_clockwork_beauty_controller (cast `/Game/Ryddelmyst_Assets/Blueprints/AI/Bestiary/ClockworkBeauty/BP_ClockworkBeautyController` (`AIBlueprintHelperLibrary.GetAIController` self)))
  (`BlackboardComponent.SetValueAsBool` (`AIBlueprintHelperLibrary.GetBlackboard` _asbp_clockwork_beauty_controller) (`self.BlasterBoltCharged`) true))

(fn `FireBlasterBolt`
  (bind _returnvalue (`|SpawnActorFromClass` "/Game/Ryddelmyst_Assets/Blueprints/AI/Bestiary/ClockworkBeauty/BP_BeautyBolt2.BP_BeautyBolt2_C" (`KismetMathLibrary.MakeTransform` (+ (`KismetMathLibrary.GreaterGreater_VectorRotator` (`KismetMathLibrary.MakeVector` 250.0) (`KismetMathLibrary.MakeRotator` (.roll (.rotation (`self.GetTransform`))) (.pitch (.rotation (`self.GetTransform`))) (.yaw (.rotation (`self.GetTransform`))))) (.location (`self.GetTransform`))) (`KismetMathLibrary.MakeRotator` (.roll (.rotation (`self.GetTransform`))) (+ (.pitch (.rotation (`self.GetTransform`))) 0.0) (.yaw (.rotation (`self.GetTransform`)))) (.scale (`self.GetTransform`))) "Undefined" "MultiplyWithRoot" null null))
  (`ProjectileMovementComponent.SetVelocityInLocalSpace` (`SpellBullet.BulletMovement` _returnvalue) (`KismetMathLibrary.MakeVector` 0.0))
  (bind _returnvalue_2 (message `Attacker.GetWeapon` (`SpellBullet.BulletMesh` _returnvalue)))
  (bind _returnvalue_3 (`BattleStatsBearer.GetStats`))
  (set `Weapon.WielderData` (`BattleStats.StatsData` _returnvalue_3) _returnvalue_2)
  (bind _asbp_clockwork_beauty_controller (cast `/Game/Ryddelmyst_Assets/Blueprints/AI/Bestiary/ClockworkBeauty/BP_ClockworkBeautyController` (`self.GetController`)))
  (`BlackboardComponent.SetValueAsBool` (`AIController.Blackboard` _asbp_clockwork_beauty_controller) (`self.BlasterBoltCharged`) false)
  (`self.BlasterBoltFired`))

(fn `FireBulletSpray`
  (`KismetSystemLibrary.PrintString` "bullets should be spraying?")
  (bind _returnvalue (`|AddComponentByClass` "/Script/Ryddelmyst.SplineGuideComponent"))
  (set `SplineGuideComponent.DebugDrawSpline` true _returnvalue)
  (set `SplineGuideComponent.DestroySpline` true _returnvalue)
  (set `SplineGuideComponent.BulletTemplate` "/Game/Ryddelmyst_Assets/Blueprints/AI/Bestiary/ClockworkBeauty/BP_BeautyFlames.BP_BeautyFlames_C" _returnvalue)
  (bind _returnvalue_2 (`AddComponent|NODE_AddSplineComponent-0`))
  (set `SplineGuideComponent.Spline` _returnvalue_2 _returnvalue)
  (`SplineGuideComponent.BuildSpline` _returnvalue)
  (`SplineGuideComponent.StartSplineBullets` _returnvalue))

(fn `FireJudgementRay`
  (`KismetSystemLibrary.PrintString` "firin' the laser!"))

(fn `GenerateDescription`
  (returns (ReturnValue :type "Descriptor Structure"))
  (locals (Descriptor :type "Descriptor Structure") (PlayerReaction :type "InteractReactions Enum") (InteractionIndex :type Integer))
  (bind _descriptions (`self.Descriptions`))
  (bind _output_get (set `local.InteractionIndex` (`KismetMathLibrary.RandomIntegerInRange` 0 (- (`KismetArrayLibrary.Array_Length` _descriptions) 1))))
  (switch `int` _output_get
    (:`Default`
      (set `local.PlayerReaction` "HAPPY"))
    (:`0`
      (set `local.PlayerReaction` "FLIRTY"))
    (:`1`
      (set `local.PlayerReaction` "EMBARRASSED"))
    (:`2`
      (set `local.PlayerReaction` "CONFUSED"))
    (:`3`
      (set `local.PlayerReaction` "ELDRITCH")))
  (bind _structout (setmembers `Descriptor` :`StructRef` (`local.Descriptor`) :`LocalizedDescription` (`|GetArrayItem` _descriptions _output_get) :`Reaction` (`local.PlayerReaction`)))
  (return _structout))

(fn `OnInteract`
  (params (Interactor :type "Actor Object Reference"))
  (returns (ReturnValue :type "Array of InteractCapability Enum"))
  (return (`self.InteractCaps`)))

(fn `UserConstructionScript`)