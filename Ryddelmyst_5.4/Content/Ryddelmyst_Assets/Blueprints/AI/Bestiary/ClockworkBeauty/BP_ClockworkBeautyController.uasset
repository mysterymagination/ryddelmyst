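; AI controller for the Clockwork Beauty enemy, handling player detection and target memory.
; On possession it runs the behavior tree and marks blaster bolt and bullet spray attacks as charged.
; Sighting a player-tagged actor cancels the forget timer, sets the prey blackboard keys and plays a random voice line at SFX volume.
; Any other perception update starts a line-of-sight timer that clears the prey when it expires.
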(event `self.ReceivePossess`
  (params (PossessedPawn :type "Pawn Object Reference"))
  (bind _blackboard (`self.Blackboard`))
  (`self.RunBehaviorTree` "/Game/Ryddelmyst_Assets/Blueprints/AI/Bestiary/ClockworkBeauty/BT_ClockworkBeautyBehavior.BT_ClockworkBeautyBehavior")
  (`BlackboardComponent.SetValueAsBool` _blackboard (`self.BlasterBoltChargedKey`) true)
  (`BlackboardComponent.SetValueAsBool` _blackboard (`self.BulletSprayChargedKey`) true))

(event `self.AIPerception.OnTargetPerceptionUpdated`
  (params (Actor :type "Actor Object Reference") (Stimulus :type "AIStimulus Structure"))
  (bind _blackboard (`self.Blackboard`))
  (bind _returnvalue (`self.K2_GetActorLocation` (`self.K2_GetPawn`)))
  (if (and (`self.ActorHasTag` Actor "Player") (`.bSuccessfullySensed` (break `AIStimulus` Stimulus)))
    (`KismetSystemLibrary.K2_ClearAndInvalidateTimerHandle` (`self.EnemyTimer`))
    (`BlackboardComponent.SetValueAsBool` _blackboard (`self.IsPreySighted`) true)
    (`BlackboardComponent.SetValueAsObject` _blackboard (`self.Prey`) Actor)
    (bind _asryddelmyst_game_instance (cast `RyddelmystGameInstance` (`GameplayStatics.GetGameInstance`)))
    (switch `int` (`KismetMathLibrary.RandomInteger` 5)
      (:`Default`
        (bind _sfxvolumescale (`RyddelmystGameInstance.SFXVolumeScale` _asryddelmyst_game_instance))
        (`GameplayStatics.PlaySoundAtLocation` "/Game/Ryddelmyst_Assets/Audio/SFX/Monsters/clockworkbeauty/UnitReady.UnitReady" _returnvalue (struct) _sfxvolumescale 1.0 0.0 null null null null :!label _label))
      (:`0`
        (`GameplayStatics.PlaySoundAtLocation` "/Game/Ryddelmyst_Assets/Audio/SFX/Monsters/clockworkbeauty/UnitUnderAttack.UnitUnderAttack" _returnvalue (struct) _sfxvolumescale 1.0 0.0 null null null null))
      (:`1`
        (`GameplayStatics.PlaySoundAtLocation` "/Game/Ryddelmyst_Assets/Audio/SFX/Monsters/clockworkbeauty/EnemiesApproaching.EnemiesApproaching" _returnvalue (struct) _sfxvolumescale 1.0 0.0 null null null null))
      (:`2`
        (`GameplayStatics.PlaySoundAtLocation` "/Game/Ryddelmyst_Assets/Audio/SFX/Monsters/clockworkbeauty/EnemyDominating.EnemyDominating" _returnvalue (struct) _sfxvolumescale 1.0 0.0 null null null null))
      (:`3`
        (`GameplayStatics.PlaySoundAtLocation` "/Game/Ryddelmyst_Assets/Audio/SFX/Monsters/clockworkbeauty/UpgradeComplete.UpgradeComplete" _returnvalue (struct) _sfxvolumescale 1.0 0.0 null null null null))
      (:`4`
        (goto _label)))
    (else
      (bind _returnvalue_2 (`KismetSystemLibrary.K2_SetTimerDelegate` (delegate `Start Enemy Timer`) (`self.Line of Sight Timer`)))
      (set `self.EnemyTimer` _returnvalue_2))))

(event `Start Enemy Timer`
  (bind _blackboard (`self.Blackboard`))
  (`BlackboardComponent.SetValueAsBool` _blackboard (`self.IsPreySighted`) false)
  (`BlackboardComponent.SetValueAsObject` _blackboard (`self.Prey`) null))

(fn `UserConstructionScript`)