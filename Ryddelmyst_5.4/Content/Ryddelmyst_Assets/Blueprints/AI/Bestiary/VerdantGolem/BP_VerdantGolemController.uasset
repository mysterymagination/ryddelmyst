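; AI controller for the Verdant Golem that runs its behavior tree and tracks the player as prey.
; On possess it starts the tree and clears the boulder and fire breath range flags on the blackboard.
; Sensing a Player-tagged actor sets the prey keys and plays stone and creak sounds.
; Any other perception update starts a line-of-sight timer that clears the prey unless the player is sensed again first.
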(event `self.ReceivePossess`
  (params (PossessedPawn :type "Pawn Object Reference"))
  (bind _blackboard (`self.Blackboard`))
  (`self.RunBehaviorTree` "/Game/Ryddelmyst_Assets/Blueprints/AI/Bestiary/VerdantGolem/BT_VerdantGolemBehavior.BT_VerdantGolemBehavior")
  (`BlackboardComponent.SetValueAsBool` _blackboard (`self.IsPreyInBoulderRange`) false)
  (`BlackboardComponent.SetValueAsBool` _blackboard (`self.IsPreyInFireBreathRange`) false))

(event `self.ReceiveTick`
  (params (DeltaSeconds :type "Float (single-precision)")))

(event `self.AIPerception.OnTargetPerceptionUpdated`
  (params (Actor :type "Actor Object Reference") (Stimulus :type "AIStimulus Structure"))
  (bind _blackboard (`self.Blackboard`))
  (bind _returnvalue (`self.K2_GetActorLocation` (`self.K2_GetPawn`)))
  (if (and (`self.ActorHasTag` Actor "Player") (`.bSuccessfullySensed` (break `AIStimulus` Stimulus)))
    (`KismetSystemLibrary.K2_ClearAndInvalidateTimerHandle` (`self.EnemyTimer`))
    (`BlackboardComponent.SetValueAsBool` _blackboard (`self.IsPreySighted`) true)
    (`BlackboardComponent.SetValueAsObject` _blackboard (`self.Prey`) Actor)
    (`GameplayStatics.PlaySoundAtLocation` "/Game/Ryddelmyst_Assets/Audio/SFX/Monsters/stone_door.stone_door" _returnvalue (struct) 1.0 1.0 0.0 null null null null)
    (`GameplayStatics.PlaySoundAtLocation` "/Game/Ryddelmyst_Assets/Audio/SFX/Monsters/tree_creak.tree_creak" _returnvalue (struct) 1.0 1.0 0.0 null null null null)
    (`KismetSystemLibrary.PrintString` (`KismetStringLibrary.Concat_StrStr` "the Prey says " (`KismetSystemLibrary.GetDisplayName` Actor)))
    (else
      (bind _returnvalue_2 (`KismetSystemLibrary.K2_SetTimerDelegate` (delegate `Start Enemy Timer`) (`self.Line of Sight Timer`)))
      (set `self.EnemyTimer` _returnvalue_2))))

(event `Start Enemy Timer`
  (bind _blackboard (`self.Blackboard`))
  (`BlackboardComponent.SetValueAsBool` _blackboard (`self.IsPreySighted`) false)
  (`BlackboardComponent.SetValueAsObject` _blackboard (`self.Prey`) null))

(fn `UserConstructionScript`)