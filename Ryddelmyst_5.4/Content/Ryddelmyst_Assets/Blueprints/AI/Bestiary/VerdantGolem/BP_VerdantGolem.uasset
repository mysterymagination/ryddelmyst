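; Verdant Golem enemy with two ranged attacks aimed at the prey actor from its AI controller's blackboard: boulder hurl and woodfire breath.
; HurlBoulder spawns a projectile, launches it toward the prey and gives its weapon message the golem's stats.
; ExhaleWoodfirebreath plays sounds and spawns Niagara particles carrying the attack, source and target.
; The breath cone tilts by the vertical offset from mouth to prey, deriving forward reach from fixed range.
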(fn `ExhaleWoodfirebreath`
  (locals (PreyKey :type Name :default "Prey") (ParticleSpawnXOffset :type "Float (double-precision)" :default 200.0) (`World Diff` :type "Vector Structure") (`Breath X Component` :type "Float (double-precision)") (`Breath Z Component` :type "Float (double-precision)") (NiagaraSystem :type "NiagaraComponent Object Reference"))
  (bind _niagarasystem (`local.NiagaraSystem`))
  (bind _returnvalue (`BlackboardComponent.GetValueAsObject` (`AIBlueprintHelperLibrary.GetBlackboard` null) (`local.PreyKey`)))
  ;[1 1 1] Validity check for controller and target actor 'prey'; if we're all ready we continue with spawning the breath particles and attack object
  (bind _asbp_verdant_golem_controller (cast `/Game/Ryddelmyst_Assets/Blueprints/AI/Bestiary/VerdantGolem/BP_VerdantGolemController` (`self.GetController`))
    (:`then`
      (if (and (`KismetSystemLibrary.IsValid` _asbp_verdant_golem_controller) (`KismetSystemLibrary.IsValid` _returnvalue))
        (bind _returnvalue_2 (`AddComponent|NODE_AddNiagaraComponent-0` :`RelativeTransform` (`KismetMathLibrary.MakeTransform` (`KismetMathLibrary.MakeVector` (`local.ParticleSpawnXOffset`)))))
        (set `local.NiagaraSystem` _returnvalue_2)
        (bind _asryddelmyst_game_instance (cast `RyddelmystGameInstance` (`GameplayStatics.GetGameInstance`)))
        (bind _sfxvolumescale (`RyddelmystGameInstance.SFXVolumeScale` _asryddelmyst_game_instance))
        (`GameplayStatics.PlaySoundAtLocation` "/Game/Ryddelmyst_Assets/Audio/SFX/Monsters/monster_roar.monster_roar" (`self.K2_GetActorLocation` (`GameplayStatics.GetPlayerPawn` 0)) (struct) _sfxvolumescale 1.0 0.0 null null null null)
        (`GameplayStatics.PlaySoundAtLocation` "/Game/Ryddelmyst_Assets/Audio/SFX/fire_sound_effect.fire_sound_effect" (`self.K2_GetActorLocation`) (struct) _sfxvolumescale 1.0 0.0 null null null null)
        (`NiagaraComponent.SetNiagaraVariableObject` _returnvalue_2 "User.CollisionRxObject" _returnvalue)
        (bind _asactor (cast `Actor` _returnvalue))
        ;[1 1 1] Set Breath Angle Algorithm, where we don't adjust angle of the breath to account for horizontal distance; we simply take the vertical component we need to aim down at the player and then generate the X component from known Z component combined with the known breath range magnitude.
        (bind _output_get (set `local.World Diff` (- (`self.K2_GetActorLocation` _asactor) (`SceneComponent.GetSocketLocation` (`self.Mesh`) "Mouth")))) ; Vector diff in world space between dest and source; since we're only rotating yaw we can use this Z component directly in the source's local space.
        (bind _output_get_2 (set `local.Breath Z Component` (.z _output_get)))
        (set `local.Breath X Component` (`KismetMathLibrary.Sqrt` (- (`KismetMathLibrary.Square` (`/Game/Ryddelmyst_Assets/Blueprints/AI/Bestiary/VerdantGolem/BP_VerdantGolemController.WoodFireBreathRange` _asbp_verdant_golem_controller)) (`KismetMathLibrary.Square` _output_get_2)))) ; Breath X Component becomes whatever is left over of the known full magnitude when you take away the known vertical aspect
        (`NiagaraComponent.SetNiagaraVariableFloat` _niagarasystem "User.ConeAxisX" (`local.Breath X Component`))
        (`NiagaraComponent.SetNiagaraVariableFloat` _niagarasystem "User.ConeAxisZ" (`local.Breath Z Component`))
        (`KismetSystemLibrary.LogString` (`KismetStringLibrary.Concat_StrStr` "breath cone axis:" (`KismetStringLibrary.Conv_VectorToString` (`KismetMathLibrary.MakeVector` (`local.Breath X Component`) 0.0 (`local.Breath Z Component`)))))
        (bind _returnvalue_3 (`|GenericCreateObject` "/Script/Ryddelmyst.WoodfirebreathAttack"))
        (`NiagaraComponent.SetNiagaraVariableObject` _niagarasystem "User.AttackObject" _returnvalue_3)
        (`NiagaraComponent.SetNiagaraVariableObject` _niagarasystem "User.SourceBattlerObject" self)))
    (:`CastFailed`
      (`KismetSystemLibrary.PrintString` "failed to exhale woodfirebreath; controller cast failed"))))

(fn `HurlBoulder`
  (locals (PreyKey :type Name :default "Prey") (SpawnUp :type "Float (double-precision)" :default 250.0) (SpawnForward :type "Float (double-precision)" :default 250.0))
  (bind _x (.x (`self.K2_GetActorLocation`)))
  (bind _y (.y (`self.K2_GetActorLocation`)))
  (bind _returnvalue (+ (.z (`self.K2_GetActorLocation`)) (`local.SpawnUp`)))
  (bind _returnvalue_2 (`|SpawnActorFromClass` "/Game/Ryddelmyst_Assets/Blueprints/AI/Bestiary/VerdantGolem/BP_HurledBoulder.BP_HurledBoulder_C" (`KismetMathLibrary.MakeTransform` (`KismetMathLibrary.MakeVector` (+ (.x (.location (`self.GetTransform`))) (`local.SpawnForward`)) (.y (.location (`self.GetTransform`))) (+ (.z (.location (`self.GetTransform`))) (`local.SpawnUp`))) (.rotation (`self.GetTransform`)) (.scale (`self.GetTransform`))) "Undefined" "MultiplyWithRoot" null null))
  (bind _asbp_verdant_golem_controller (cast `/Game/Ryddelmyst_Assets/Blueprints/AI/Bestiary/VerdantGolem/BP_VerdantGolemController` (`self.GetController`)))
  (bind _asactor (cast `Actor` (`BlackboardComponent.GetValueAsObject` (`AIBlueprintHelperLibrary.GetBlackboard` _asbp_verdant_golem_controller) (`local.PreyKey`))))
  (bind _returnvalue_3 (`self.K2_GetActorLocation` _asactor))
  (bind _returnvalue_4 (`KismetMathLibrary.GetDirectionUnitVector` (`KismetMathLibrary.MakeVector` _x _y _returnvalue) _returnvalue_3))
  (`ProjectileMovementComponent.SetVelocityInLocalSpace` (`SpellBullet.BulletMovement` _returnvalue_2) _returnvalue_4)
  (bind _returnvalue_5 (message `Attacker.GetWeapon` (`SpellBullet.BulletMesh` _returnvalue_2)))
  (bind _returnvalue_6 (`BattleStatsBearer.GetStats`))
  (set `Weapon.WielderData` (`BattleStats.StatsData` _returnvalue_6) _returnvalue_5)
  (`KismetSystemLibrary.PrintString` (`KismetStringLibrary.Concat_StrStr` "maya is at " (`KismetStringLibrary.Conv_VectorToString` _returnvalue_3) "and boulder is at " (`KismetStringLibrary.Conv_VectorToString` (`KismetMathLibrary.MakeVector` _x _y _returnvalue)) "so direction is " (`KismetStringLibrary.Conv_VectorToString` _returnvalue_4))))

(fn `UserConstructionScript`)