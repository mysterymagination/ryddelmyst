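; AI controller for the Reaper Treant enemy that detects and hunts the player through a behavior tree.
; On possession it starts the tree, and its perception component writes sighted prey to the Blackboard unless the treant is dying.
; Sightings play a roar or voice line at the player's location, based on the anim instance's panic flag.
; Other perception updates start an attention-span timer that clears the prey keys.
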(event `self.ReceivePossess`
  (params (PossessedPawn :type "Pawn Object Reference"))
  (`self.RunBehaviorTree` "/Game/Ryddelmyst_Assets/Blueprints/AI/Bestiary/ReaperTreant/BT_ReaperTreantBehavior.BT_ReaperTreantBehavior"))

(event `self.SnifferOfReaperTreant.OnTargetPerceptionUpdated`
  (params (Actor :type "Actor Object Reference") (Stimulus :type "AIStimulus Structure"))
  (bind (_age _expirationage _strength _stimuluslocation _receiverlocation _tag _bsuccessfullysensed) (break `AIStimulus` Stimulus))
  (bind _returnvalue (`self.K2_GetActorLocation` Actor))
  (bind _blackboard (`self.Blackboard`))
  (if (not (`BlackboardComponent.GetValueAsBool` (`self.Blackboard`) (`self.IsDying`)))
    (`KismetSystemLibrary.PrintString` (`KismetStringLibrary.Concat_StrStr` "sensed: " (`KismetStringLibrary.Conv_BoolToString` _bsuccessfullysensed)))
    (if (and (`self.ActorHasTag` Actor "Player") _bsuccessfullysensed)
      (`KismetSystemLibrary.K2_ClearAndInvalidateTimerHandle` (`self.InterestTimer`))
      (`BlackboardComponent.SetValueAsBool` _blackboard (`self.IsPreySighted`) true)
      (`BlackboardComponent.SetValueAsObject` _blackboard (`self.Prey`) Actor)
      (`KismetSystemLibrary.PrintString` "chasing maya!")
      (bind _asbp_reaper_treant (cast `/Game/Ryddelmyst_Assets/Blueprints/AI/Bestiary/ReaperTreant/BP_ReaperTreant` (`self.K2_GetPawn`)))
      (bind _asbp_reaper_treant_anim (cast `/Game/Ryddelmyst_Assets/Animations/BP_ReaperTreantAnim` (`SkeletalMeshComponent.GetAnimInstance` (`Character.Mesh` _asbp_reaper_treant))))
      (if (`/Game/Ryddelmyst_Assets/Animations/BP_ReaperTreantAnim.IsPanic` _asbp_reaper_treant_anim)
        (`GameplayStatics.PlaySoundAtLocation` "/Game/Ryddelmyst_Assets/Audio/SFX/Monsters/monster_roar.monster_roar" _returnvalue (struct) 1.0 1.0 0.0 null null null null)
        (else
          (`GameplayStatics.PlaySoundAtLocation` "/Game/Ryddelmyst_Assets/Audio/SFX/Monsters/i_see_you_voice.i_see_you_voice" _returnvalue (struct) 1.0 1.0 0.0 null null null null)))
      (else
        (bind _returnvalue_2 (`KismetSystemLibrary.K2_SetTimerDelegate` (delegate `Lose Interest`) (`self.AttentionSpan`)))
        (set `self.InterestTimer` _returnvalue_2)))))

(event `Lose Interest`
  (bind _blackboard (`self.Blackboard`))
  (`BlackboardComponent.SetValueAsBool` _blackboard (`self.IsPreySighted`) false)
  (`BlackboardComponent.SetValueAsObject` _blackboard (`self.Prey`) null)
  (`BlackboardComponent.SetValueAsBool` _blackboard (`self.IsPreyWithinReach`) false)
  (`KismetSystemLibrary.PrintString` "lost track of maya..."))

(fn `UserConstructionScript`)