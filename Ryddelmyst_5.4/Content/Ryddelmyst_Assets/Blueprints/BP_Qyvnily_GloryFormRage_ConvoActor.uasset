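; Conversation actor for Qyvnily's GloryFormRage form, giving the player reactions and descriptions of her.
; When a Player-tagged actor hits its component, it shows one of four random Maya lines with a matching portrait through the HUD.
; GenerateDescription picks text and reaction by bone name, first adding one to the Qyvnily_Forms_Visited value once, though storing it under an empty key.
; OnInteract just returns InteractCap.
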(event `self.Qyvnily_GloryFormRage.OnComponentHit`
  (params (HitComponent :type "PrimitiveComponent Object Reference") (OtherActor :type "Actor Object Reference") (OtherComp :type "PrimitiveComponent Object Reference") (NormalImpulse :type "Vector Structure") (Hit :type "HitResult Structure (by ref)"))
  (if (`self.ActorHasTag` OtherActor "Player")
    (bind _asryddelmyst_hud (cast `RyddelmystHUD` (`PlayerController.GetHUD` (`GameplayStatics.GetPlayerController` 0))))
    (switch `int` (`KismetMathLibrary.RandomIntegerInRange` 0 3)
      (:`0`
        (bind _output_get (set `self.FlirtyText` "Heeey there, girl. You look kinda smite-y..."))
        (`RyddelmystHUD.ShowDialogue` _asryddelmyst_hud "/Game/Ryddelmyst_Assets/Sprites/Maya_Flirty_Portrait_Sprite.Maya_Flirty_Portrait_Sprite" _output_get))
      (:`1`
        (bind _output_get_2 (set `self.FlirtyText` "Such stormy hair!"))
        (`RyddelmystHUD.ShowDialogue` _asryddelmyst_hud "/Game/Ryddelmyst_Assets/Sprites/Maya_Eldritch_Portrait_Sprite.Maya_Eldritch_Portrait_Sprite" _output_get_2))
      (:`2`
        (bind _output_get_3 (set `self.FlirtyText` "Did her dress get even prettier?!"))
        (`RyddelmystHUD.ShowDialogue` _asryddelmyst_hud "/Game/Ryddelmyst_Assets/Sprites/Maya_Happy_Portrait_Sprite.Maya_Happy_Portrait_Sprite" _output_get_3))
      (:`3`
        (bind _output_get_4 (set `self.FlirtyText` "Sweet rolling snowballs, her hair is glorious! I wish mine was all cape-like; I'd swish it round *whoosh* all dramatic at every entrance."))
        (`RyddelmystHUD.ShowDialogue` _asryddelmyst_hud "/Game/Ryddelmyst_Assets/Sprites/Maya_Happy_Portrait_Sprite.Maya_Happy_Portrait_Sprite" _output_get_4)))))

(fn `GenerateDescription`
  (params (BoneName :type Name))
  (returns (ReturnValue :type "Descriptor Structure"))
  (if (not (`self.EncounterCounted`))
    (bind _asryddelmyst_game_state (cast `RyddelmystGameState` (`GameplayStatics.GetGameState`)))
    (bind _statesmapint (`RyddelmystGameState.StatesMapInt` _asryddelmyst_game_state))
    (`BlueprintMapLibrary.Map_Add` _statesmapint "" (+ (`BlueprintMapLibrary.Map_Find` _statesmapint "Qyvnily_Forms_Visited") 1))
    (set `self.EncounterCounted` true))
  (switch `string` (`KismetStringLibrary.Conv_NameToString` BoneName)
    (:`Default`
      (set `self.Desc` (make `Descriptor` (`self.GeneralDesc`) (struct :`Genre` "Conversation") "ELDRITCH")))
    (:`Lady Garden`
      (set `self.Desc` (make `Descriptor` (`self.ThighsDesc`))))
    (:`Boobs`
      (set `self.Desc` (make `Descriptor` (`self.ChestDesc`) (struct :`Genre` "Conversation") "FLIRTY"))))
  (return (`self.Desc`)))

(fn `OnInteract`
  (params (Interactor :type "Actor Object Reference"))
  (returns (ReturnValue :type "Array of InteractCapability Enum"))
  (return (`self.InteractCap`)))

(fn `UserConstructionScript`)