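; BP_CracklingVioletVialItem is the Crackling Violet Vial item, a piece of equipment for the Neck slot.
; Its getters return the item's name, description and icon from its own variables for display.
; It always reports itself as equippable and hardcodes the slot name, with no effect logic in these graphs.
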(fn `GetDisplayDescription`
  (returns (ReturnValue :type Text))
  (return (`self.DisplayDesc`)))

(fn `GetDisplayIcon`
  (returns (ReturnValue :type "Texture2D Object Reference"))
  (return (`self.DisplayIcon`)))

(fn `GetDisplayName`
  (returns (ReturnValue :type Text))
  (return (`self.DisplayName`)))

(fn `GetEquipSlot`
  (returns (ReturnValue :type String))
  (return "Neck"))

(fn `IsEquippable`
  (returns (ReturnValue :type Boolean))
  (return true))