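; BP_DiaryEntry is a diary actor that supplies readable lore to the game.
; GenerateDescription packs its text, title and conversation script into a descriptor as Diary-genre library book data with a happy reaction.
; OnInteract returns its interaction capability array, and player overlap with the paper sprite plays a sound.
; ProcessStringTemplate is an unfinished variable-substitution stub whose token-search loop has an empty body.
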(event `self.PaperSprite.OnComponentBeginOverlap`
  (params (OverlappedComponent :type "PrimitiveComponent Object Reference") (OtherActor :type "Actor Object Reference") (OtherComp :type "PrimitiveComponent Object Reference") (OtherBodyIndex :type Integer) (bFromSweep :type Boolean) (SweepResult :type "HitResult Structure (by ref)"))
  (if (`self.ActorHasTag` OtherActor "Player")
    (`GameplayStatics.PlaySound2D` "/Engine/EditorSounds/Notifications/CompileSuccess.CompileSuccess" 1.0 1.0 0.0 null null)))

(fn `GenerateDescription`
  (params (BoneName :type Name))
  (returns (ReturnValue :type "Descriptor Structure"))
  (return (make `Descriptor` (`self.DescText`) (make `LibraryBookData` (`self.LoreTitle`) (`self.LoreText`) "" (`self.ConvoScript`) "Diary"))))

(fn `OnInteract`
  (params (Interactor :type "Actor Object Reference"))
  (returns (ReturnValue :type "Array of InteractCapability Enum"))
  (return (`self.InteractCapArray`)))

(fn `ProcessStringTemplate`
  (params (FormatString :type String))
  (locals (VarOpenerToken :type String :default "${") (VarEndToken :type String :default "}") (NotFoundIndex :type Integer :default -1))
  (while (!= (`KismetStringLibrary.FindSubstring` FormatString (`local.VarOpenerToken`)) (`local.NotFoundIndex`))
    _))

(fn `UserConstructionScript`)