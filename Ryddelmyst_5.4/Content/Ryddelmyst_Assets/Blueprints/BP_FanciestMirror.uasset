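; BP_FanciestMirror is an interactable mirror actor that supplies body-part-specific descriptions, each paired with a character reaction.
; GenerateDescription switches on the bone name to build a descriptor with localized text, empty lore and a reaction, with left and right limbs sharing entries.
; Unmatched bones fall back to a general, happy description.
; OnInteract simply returns its interact capability array, and the event graph and construction script are empty.
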(fn `GenerateDescription`
  (params (BoneName :type Name))
  (returns (ReturnValue :type "Descriptor Structure"))
  (switch `string` (`KismetStringLibrary.Conv_NameToString` BoneName)
    (:`Default`
      (set `self.Desc` (make `Descriptor` (`self.GeneralDesc`))))
    (:`Boobs`
      (set `self.Desc` (make `Descriptor` (`self.BoobDesc`) "" "FLIRTY")))
    (:`Face`
      (set `self.Desc` (make `Descriptor` (`self.FaceDesc`) "" "CONFUSED")))
    (:`Legs_L`
      (set `self.Desc` (make `Descriptor` (`self.LegDesc`) "" "FLIRTY") :!label _label))
    (:`Legs_R`
      (goto _label))
    (:`Shoulder_L`
      (set `self.Desc` (make `Descriptor` (`self.ShoulderDesc`) "" "EMBARRASSED") :!label _label_2))
    (:`Shoulder_R`
      (goto _label_2))
    (:`Hips_L`
      (set `self.Desc` (make `Descriptor` (`self.HipDesc`) "" "FLIRTY") :!label _label_3))
    (:`Hips_R`
      (goto _label_3))
    (:`Thighs_L`
      (set `self.Desc` (make `Descriptor` (`self.ThighDesc`) "" "FLIRTY") :!label _label_4))
    (:`Thighs_R`
      (goto _label_4))
    (:`Feet`
      (set `self.Desc` (make `Descriptor` (`self.ShoesDesc`) "" "CONFUSED")))
    (:`Lady Garden`
      (set `self.Desc` (make `Descriptor` (`self.LadyGardenDesc`) "" "CONFUSED")))
    (:`Dress`
      (set `self.Desc` (make `Descriptor` (`self.DressDesc`) "" "FLIRTY")))
    (:`Hat`
      (set `self.Desc` (make `Descriptor` (`self.HatDesc`) "" "CONFUSED")))
    (:`Hair`
      (set `self.Desc` (make `Descriptor` (`self.HairDesc`) "" "ELDRITCH")))
    (:`Arm_L`
      (set `self.Desc` (make `Descriptor` (`self.ArmDesc`)) :!label _label_5))
    (:`Arm_R`
      (goto _label_5)))
  (return (`self.Desc`)))

(fn `OnInteract`
  (params (Interactor :type "Actor Object Reference"))
  (returns (ReturnValue :type "Array of InteractCapability Enum"))
  (return (`self.InteractCapArray`)))

(fn `UserConstructionScript`)