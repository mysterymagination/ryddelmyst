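; BP_QyvnilyConvo_WildFormActor is the interactable actor for Qyvnily's wild form, reacting to player contact and supplying descriptions of the character.
; When the player bumps its Qyvnily_WildForm component, it shows one of three random flirty lines with a matching Maya portrait through RyddelmystHUD.
; GenerateDescription maps the given bone name to body-part-specific text and a reaction, with a general fallback.
; OnInteract returns its array of interaction capabilities.
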(event `self.Qyvnily_WildForm.OnComponentHit`
  (params (HitComponent :type "PrimitiveComponent Object Reference") (OtherActor :type "Actor Object Reference") (OtherComp :type "PrimitiveComponent Object Reference") (NormalImpulse :type "Vector Structure") (Hit :type "HitResult Structure (by ref)"))
  (if (`self.ActorHasTag` OtherActor "Player")
    (bind _asryddelmyst_hud (cast `RyddelmystHUD` (`PlayerController.GetHUD` (`GameplayStatics.GetPlayerController` 0))))
    (switch `int` (`KismetMathLibrary.RandomIntegerInRange` 0 2)
      (:`0`
        (bind _output_get (set `self.FlirtyText` "Brr, suddenly got quite chilly!"))
        (`RyddelmystHUD.ShowDialogue` _asryddelmyst_hud "/Game/Ryddelmyst_Assets/Textures/maya_portraits_Sprite_Sad.maya_portraits_Sprite_Sad" _output_get))
      (:`1`
        (bind _output_get_2 (set `self.FlirtyText` "Oh wow, pointy. Her myriad ice spikes are pointy too."))
        (`RyddelmystHUD.ShowDialogue` _asryddelmyst_hud "/Game/Ryddelmyst_Assets/Textures/maya_portraits_Sprite_Eldritch.maya_portraits_Sprite_Eldritch" _output_get_2))
      (:`2`
        (bind _output_get_3 (set `self.FlirtyText` "Whoa hello snow woman! Hmm, her ice crystals are squishier than they look."))
        (`RyddelmystHUD.ShowDialogue` _asryddelmyst_hud "/Game/Ryddelmyst_Assets/Textures/maya_portraits_Sprite_Embarrassed.maya_portraits_Sprite_Embarrassed" _output_get_3)))))

(fn `GenerateDescription`
  (params (BoneName :type Name))
  (returns (ReturnValue :type "Descriptor Structure"))
  (switch `name` BoneName
    (:`Default`
      (set `self.Desc` (make `Descriptor` (`self.GeneralDesc`))))
    (:`Face`
      (set `self.Desc` (make `Descriptor` (`self.FaceDesc`) "" "SAD")))
    (:`Boobs`
      (set `self.Desc` (make `Descriptor` (`self.BoobsDesc`) "" "EMBARRASSED")))
    (:`Lady Garden`
      (set `self.Desc` (make `Descriptor` (`self.LadyGardenDesc`) "" "ELDRITCH"))))
  (return (`self.Desc`)))

(fn `OnInteract`
  (params (Interactor :type "Actor Object Reference"))
  (returns (ReturnValue :type "Array of InteractCapability Enum"))
  (return (`self.InteractCapArray`)))

(fn `UserConstructionScript`)