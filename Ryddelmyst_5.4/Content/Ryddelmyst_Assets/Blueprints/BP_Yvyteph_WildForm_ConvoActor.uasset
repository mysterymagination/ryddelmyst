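; Conversation actor for Yvyteph's wild form that supplies flirtatious reactions and inspectable descriptions.
; When a player-tagged actor hits its S_Yvyteph_WildForm component, it shows one of three random Maya lines with a matching portrait through the Ryddelmyst HUD.
; GenerateDescription maps the bone name to a localized body-part description and reaction, falling back to a general one.
; OnInteract simply returns its InteractCapArray.
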(event `self.S_Yvyteph_WildForm.OnComponentHit`
  (params (HitComponent :type "PrimitiveComponent Object Reference") (OtherActor :type "Actor Object Reference") (OtherComp :type "PrimitiveComponent Object Reference") (NormalImpulse :type "Vector Structure") (Hit :type "HitResult Structure (by ref)"))
  (if (`KismetSystemLibrary.IsValid` OtherActor)
    (if (`self.ActorHasTag` OtherActor "Player")
      (bind _asryddelmyst_hud (cast `RyddelmystHUD` (`PlayerController.GetHUD` (`GameplayStatics.GetPlayerController` 0))))
      (switch `int` (`KismetMathLibrary.RandomIntegerInRange` 0 2)
        (:`0`
          (bind _output_get (set `self.FlirtyText` "Did it just get hot in here?"))
          (`RyddelmystHUD.ShowDialogue` _asryddelmyst_hud "/Game/Ryddelmyst_Assets/Textures/maya_portraits_Sprite_Eldritch.maya_portraits_Sprite_Eldritch" _output_get))
        (:`1`
          (bind _output_get_2 (set `self.FlirtyText` "Yep, no problem worshipping her <3"))
          (`RyddelmystHUD.ShowDialogue` _asryddelmyst_hud "/Game/Ryddelmyst_Assets/Textures/maya_portraits_Sprite_Flirty.maya_portraits_Sprite_Flirty" _output_get_2))
        (:`2`
          (bind _output_get_3 (set `self.FlirtyText` "Does this count as a meet-cute? Please say it does!"))
          (`RyddelmystHUD.ShowDialogue` _asryddelmyst_hud "/Game/Ryddelmyst_Assets/Textures/maya_portraits_Sprite_Happy.maya_portraits_Sprite_Happy" _output_get_3))))))

(fn `GenerateDescription`
  (params (BoneName :type Name))
  (returns (ReturnValue :type "Descriptor Structure"))
  (switch `name` BoneName
    (:`Default`
      (set `self.Desc` (make `Descriptor` (`self.GeneralDesc`))))
    (:`Face`
      (set `self.Desc` (make `Descriptor` (`self.FaceDesc`) (struct :`Genre` "Conversation") "SAD")))
    (:`Boobs`
      (set `self.Desc` (make `Descriptor` (`self.BoobsDesc`) (struct :`Genre` "Conversation") "FLIRTY")))
    (:`Lady Garden`
      (set `self.Desc` (make `Descriptor` (`self.LadyGardenDesc`) (struct :`Genre` "Conversation") "CONFUSED"))))
  (return (`self.Desc`)))

(fn `OnInteract`
  (params (Interactor :type "Actor Object Reference"))
  (returns (ReturnValue :type "Array of InteractCapability Enum"))
  (return (`self.InteractCapArray`)))

(fn `UserConstructionScript`)