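; Conversation actor for Qyvnily's wild form, an ice-spiked woman the player can bump into, inspect and interact with.
; Player collisions show one of three random flirty Maya lines with portraits on the HUD.
; GenerateDescription picks text and reaction by bone, then plays a volume-scaled cackle.
; Its first call flags the encounter and reads the Qyvnily_Forms_Visited count, but stores the increment under an empty key.
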(event `self.Qyvnily_WildForm.OnComponentHit`
  (params (HitComponent :type "PrimitiveComponent Object Reference") (OtherActor :type "Actor Object Reference") (OtherComp :type "PrimitiveComponent Object Reference") (NormalImpulse :type "Vector Structure") (Hit :type "HitResult Structure (by ref)"))
  (if (`self.ActorHasTag` OtherActor "Player")
    (bind _asryddelmyst_hud (cast `RyddelmystHUD` (`PlayerController.GetHUD` (`GameplayStatics.GetPlayerController` 0))))
    (switch `int` (`KismetMathLibrary.RandomIntegerInRange` 0 2)
      (:`0`
        (bind _output_get (set `self.FlirtyText` "Brr, suddenly got quite chilly!"))
        (`RyddelmystHUD.ShowDialogue` _asryddelmyst_hud "/Game/Ryddelmyst_Assets/Sprites/Maya_Sad_Portrait_Sprite.Maya_Sad_Portrait_Sprite" _output_get))
      (:`1`
        (bind _output_get_2 (set `self.FlirtyText` "Oh wow, pointy. Her myriad ice spikes are pointy too."))
        (`RyddelmystHUD.ShowDialogue` _asryddelmyst_hud "/Game/Ryddelmyst_Assets/Sprites/Maya_Eldritch_Portrait_Sprite.Maya_Eldritch_Portrait_Sprite" _output_get_2))
      (:`2`
        (bind _output_get_3 (set `self.FlirtyText` "Whoa hello snow woman! Hmm, her ice crystals are squishier than they look."))
        (`RyddelmystHUD.ShowDialogue` _asryddelmyst_hud "/Game/Ryddelmyst_Assets/Sprites/Maya_Embarrassed_Portrait_Sprite.Maya_Embarrassed_Portrait_Sprite" _output_get_3)))))

(fn `GenerateDescription`
  (params (BoneName :type Name))
  (returns (ReturnValue :type "Descriptor Structure"))
  (if (not (`self.EncounterCounted`))
    (bind _asryddelmyst_game_state (cast `RyddelmystGameState` (`GameplayStatics.GetGameState`)))
    (bind _statesmapint (`RyddelmystGameState.StatesMapInt` _asryddelmyst_game_state))
    (`BlueprintMapLibrary.Map_Add` _statesmapint "" (+ (`BlueprintMapLibrary.Map_Find` _statesmapint "Qyvnily_Forms_Visited") 1))
    (set `self.EncounterCounted` true))
  (switch `name` BoneName
    (:`Default`
      (set `self.Desc` (make `Descriptor` (`self.GeneralDesc`))))
    (:`Boobs`
      (set `self.Desc` (make `Descriptor` (`self.BoobsDesc`) (struct :`Genre` "Observation") "EMBARRASSED")))
    (:`Lady Garden`
      (set `self.Desc` (make `Descriptor` (`self.LadyGardenDesc`) (struct :`Genre` "Observation") "ELDRITCH"))))
  (bind _asryddelmyst_game_instance (cast `RyddelmystGameInstance` (`GameplayStatics.GetGameInstance`))
    (:`then`
      (`GameplayStatics.PlaySoundAtLocation` "/Game/Ryddelmyst_Assets/Audio/VO/Maya/evil_cackle_laugh_2.evil_cackle_laugh_2" (`self.K2_GetActorLocation`) (struct) (`RyddelmystGameInstance.SFXVolumeScale` _asryddelmyst_game_instance) 1.0 0.0 null null null null))
    (:`CastFailed`
      _))
  (return (`self.Desc`)))

(fn `OnInteract`
  (params (Interactor :type "Actor Object Reference"))
  (returns (ReturnValue :type "Array of InteractCapability Enum"))
  (return (`self.InteractCapArray`)))

(fn `UserConstructionScript`)