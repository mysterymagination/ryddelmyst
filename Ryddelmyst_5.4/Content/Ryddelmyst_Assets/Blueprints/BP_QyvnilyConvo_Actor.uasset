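; Conversation actor for Qyvnily's wildflower form, providing Maya's bump reactions and inspection descriptions.
; Player hits on the flower component show one of five random flirty lines with a portrait through the Ryddelmyst HUD.
; GenerateDescription maps bone names to localized descriptions and reactions; its first call increments the Qyvnily forms-visited count, but writes it under an empty key.
; OnInteract simply returns the interaction capability array.
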(event `self.Qyvnily_WildFlower.OnComponentHit`
  (params (HitComponent :type "PrimitiveComponent Object Reference") (OtherActor :type "Actor Object Reference") (OtherComp :type "PrimitiveComponent Object Reference") (NormalImpulse :type "Vector Structure") (Hit :type "HitResult Structure (by ref)"))
  (if (`self.ActorHasTag` OtherActor "Player")
    (bind _asryddelmyst_hud (cast `RyddelmystHUD` (`PlayerController.GetHUD` (`GameplayStatics.GetPlayerController` 0))))
    (switch `int` (`KismetMathLibrary.RandomIntegerInRange` 0 4)
      (:`0`
        (bind _output_get (set `self.FlirtyText` "Good gravy girl, have you felt your hair?! You're like a chinchilla made of cloud :3 Now I have to wonder if the carpet matches the curtains..."))
        (`RyddelmystHUD.ShowDialogue` _asryddelmyst_hud "/Game/Ryddelmyst_Assets/Textures/maya_portraits_Sprite_Flirty.maya_portraits_Sprite_Flirty" _output_get))
      (:`1`
        (bind _output_get_2 (set `self.FlirtyText` "Ooh hey, even the leaves of her bottoms are silky soft!"))
        (`RyddelmystHUD.ShowDialogue` _asryddelmyst_hud "/Game/Ryddelmyst_Assets/Textures/maya_portraits_Sprite_Flirty.maya_portraits_Sprite_Flirty" _output_get_2))
      (:`2`
        (bind _output_get_3 (set `self.FlirtyText` "Hi five!"))
        (`RyddelmystHUD.ShowDialogue` _asryddelmyst_hud "/Game/Ryddelmyst_Assets/Textures/maya_portraits_Sprite_Flirty.maya_portraits_Sprite_Flirty" _output_get_3))
      (:`3`
        (bind _output_get_4 (set `self.FlirtyText` "Sweet toplessness, and she called me girlfish! What an honor!"))
        (`RyddelmystHUD.ShowDialogue` _asryddelmyst_hud "/Game/Ryddelmyst_Assets/Textures/maya_portraits_Sprite_Flirty.maya_portraits_Sprite_Flirty" _output_get_4))
      (:`4`
        (bind _output_get_5 (set `self.FlirtyText` "HUGS <3"))
        (`RyddelmystHUD.ShowDialogue` _asryddelmyst_hud "/Game/Ryddelmyst_Assets/Textures/maya_portraits_Sprite_Flirty.maya_portraits_Sprite_Flirty" _output_get_5)))))

(fn `GenerateDescription`
  (params (BoneName :type Name))
  (returns (ReturnValue :type "Descriptor Structure"))
  (if (not (`self.EncounterCounted`))
    (bind _asryddelmyst_game_state (cast `RyddelmystGameState` (`GameplayStatics.GetGameState`)))
    (bind _statesmapint (`RyddelmystGameState.StatesMapInt` _asryddelmyst_game_state))
    (`BlueprintMapLibrary.Map_Add` _statesmapint "" (+ (`BlueprintMapLibrary.Map_Find` _statesmapint "Qyvnily_Forms_Visited") 1))
    (set `self.EncounterCounted` true))
  (switch `name` BoneName
    (:`Default`
      (set `self.Desc` (make `Descriptor` (`self.GeneralDesc`))))
    (:`Face`
      (set `self.Desc` (make `Descriptor` (`self.FaceDesc`))))
    (:`Boobs`
      (set `self.Desc` (make `Descriptor` (`self.BoobsDesc`) (struct :`Genre` "Conversation") "ELDRITCH")))
    (:`Lady Garden`
      (set `self.Desc` (make `Descriptor` (`self.LadyGardenDesc`)))))
  (return (`self.Desc`)))

(fn `OnInteract`
  (params (Interactor :type "Actor Object Reference"))
  (returns (ReturnValue :type "Array of InteractCapability Enum"))
  (return (`self.InteractCapArray`)))

(fn `UserConstructionScript`)