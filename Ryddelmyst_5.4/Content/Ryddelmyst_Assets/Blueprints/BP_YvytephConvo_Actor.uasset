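; Interactable actor for Yvyteph, whose Font of Fertility mesh triggers character dialogue when the player bumps into or examines it.
; Player hits show one of several random portrait-and-text lines through RyddelmystHUD, with one roll left silent.
; GenerateDescription maps the given bone name to a localized description and emotional reaction, falling back to a general one.
; OnInteract simply returns the InteractCapArray.
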(event `self.S_Yvyteph_FontOfFertility.OnComponentHit`
  (params (HitComponent :type "PrimitiveComponent Object Reference") (OtherActor :type "Actor Object Reference") (OtherComp :type "PrimitiveComponent Object Reference") (NormalImpulse :type "Vector Structure") (Hit :type "HitResult Structure (by ref)"))
  (if (`self.ActorHasTag` OtherActor "Player")
    (bind _asryddelmyst_hud (cast `RyddelmystHUD` (`PlayerController.GetHUD` (`GameplayStatics.GetPlayerController` 0))))
    (switch `int` (`KismetMathLibrary.RandomIntegerInRange` 0 4)
      (:`0`
        (bind _output_get (set `self.FlirtyText` "Ooh wow, that squish. I need a lie down."))
        (`RyddelmystHUD.ShowDialogue` _asryddelmyst_hud "/Game/Ryddelmyst_Assets/Textures/maya_portraits_Sprite_Flirty.maya_portraits_Sprite_Flirty" _output_get))
      (:`1`
        (bind _output_get_2 (set `self.FlirtyText` "Oop, sorry Mistress. I didn't mean to touch your... well, everything. There really isn't a safe place to collide with you in this form."))
        (`RyddelmystHUD.ShowDialogue` _asryddelmyst_hud "/Game/Ryddelmyst_Assets/Textures/maya_portraits_Sprite_Confused.maya_portraits_Sprite_Confused" _output_get_2))
      (:`2`
        (bind _output_get_3 (set `self.FlirtyText` "Yep, no problem worshipping her <3"))
        (`RyddelmystHUD.ShowDialogue` _asryddelmyst_hud "/Game/Ryddelmyst_Assets/Textures/maya_portraits_Sprite_Flirty.maya_portraits_Sprite_Flirty" _output_get_3))
      (:`4`
        (bind _output_get_4 (set `self.FlirtyText` "Her bark is surprisingly soft. Supple. Neat! "))
        (`RyddelmystHUD.ShowDialogue` _asryddelmyst_hud "/Game/Ryddelmyst_Assets/Textures/maya_portraits_Sprite_Happy.maya_portraits_Sprite_Happy" _output_get_4)))))

(fn `GenerateDescription`
  (params (BoneName :type Name))
  (returns (ReturnValue :type "Descriptor Structure"))
  (switch `name` BoneName
    (:`Default`
      (set `self.Desc` (make `Descriptor` (`self.GeneralDesc`) (struct :`Genre` "Conversation") "FLIRTY")))
    (:`Face`
      (set `self.Desc` (make `Descriptor` (`self.FaceDesc`) (struct :`Genre` "Conversation") "SAD")))
    (:`Boobs`
      (set `self.Desc` (make `Descriptor` (`self.BoobsDesc`) (struct :`Genre` "Conversation") "CONFUSED")))
    (:`Lady Garden`
      (set `self.Desc` (make `Descriptor` (`self.LadyGardenDesc`) (struct :`Genre` "Conversation") "ELDRITCH"))))
  (return (`self.Desc`)))

(fn `OnInteract`
  (params (Interactor :type "Actor Object Reference"))
  (returns (ReturnValue :type "Array of InteractCapability Enum"))
  (return (`self.InteractCapArray`)))

(fn `UserConstructionScript`)