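; BP_ChromeKeyItem is an item Blueprint, named as a chrome key, that supplies display and equip data through getter functions.
; It returns its icon and description from the DisplayIcon and DisplayDesc variables.
; It reports itself as not equippable with an empty equip slot, and its display name getter also returns an empty string.
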(fn `GetDisplayDescription`
  (returns (ReturnValue :type Text))
  (return (`self.DisplayDesc`)))

(fn `GetDisplayIcon`
  (returns (ReturnValue :type "Texture2D Object Reference"))
  (return (`self.DisplayIcon`)))

(fn `GetDisplayName`
  (returns (ReturnValue :type Text))
  (return ""))

(fn `GetEquipSlot`
  (returns (ReturnValue :type String))
  (return ""))

(fn `IsEquippable`
  (returns (ReturnValue :type Boolean))
  (return false))