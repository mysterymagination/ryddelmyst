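; BP_MollyStatue is an interactable statue that supplies a description and character reaction when looked at.
; GenerateDescription fills a Descriptor struct with the main description and a confused reaction on first look, then clears the first-look flag.
; Later looks use a second-look description with a random happy, flirty, embarrassed or confused reaction.
; OnInteract only prints the main description and returns its interaction capability array.
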(fn `GenerateDescription`
  (returns (ReturnValue :type "Descriptor Structure"))
  (locals (RandoReact :type "InteractReactions Enum"))
  (bind _descriptor (`self.Descriptor`))
  (if (`self.IsFirstLook`)
    (bind _structout (setmembers `Descriptor` :`StructRef` _descriptor :`LocalizedDescription` (`self.Description`) :`Reaction` "CONFUSED"))
    (else
      (switch `int` (`KismetMathLibrary.RandomIntegerInRange` 0 3)
        (:`0`
          (set `local.RandoReact` "HAPPY"))
        (:`1`
          (set `local.RandoReact` "FLIRTY"))
        (:`2`
          (set `local.RandoReact` "EMBARRASSED"))
        (:`3`
          (set `local.RandoReact` "CONFUSED")))
      (setmembers `Descriptor` :`StructRef` _descriptor :`LocalizedDescription` (`self.SecondLookDesc`) :`Reaction` (`local.RandoReact`))))
  (set `self.IsFirstLook` false)
  (return _structout))

(fn `OnInteract`
  (params (Interactor :type "Actor Object Reference"))
  (returns (ReturnValue :type "Array of InteractCapability Enum"))
  (`KismetSystemLibrary.PrintString` (`KismetTextLibrary.Conv_TextToString` (`self.Description`)))
  (return (`self.InteractCapArray`)))

(fn `UserConstructionScript`)