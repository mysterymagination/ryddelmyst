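; BP_WoodEgg is an interactable wooden egg that is destroyed when it overlaps a lapping lava pool.
; On that overlap it fires the game instance event manager's WoodEggDeath event with its location, spawns a kill effect, plays an explosion scaled by SFX volume, and destroys itself.
; OnInteract only prints a debug string and returns its interaction capability array.
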(event `self.ReceiveActorBeginOverlap`
  (params (OtherActor :type "Actor Object Reference"))
  (bind _returnvalue (`self.K2_GetActorLocation`))
  (cast `/Game/Ryddelmyst_Assets/Blueprints/BP_LappingLavaPool` OtherActor)
  (`KismetSystemLibrary.PrintString` "oh god fire pool!")
  (bind _asryddelmyst_game_instance (cast `RyddelmystGameInstance` (`GameplayStatics.GetGameInstance`)))
  (bind _returnvalue_2 (`RyddelmystGameInstance.GetEventManager` _asryddelmyst_game_instance))
  (`RyddelmystEventManager.WoodEggDeathEvent` _returnvalue_2 _returnvalue)
  (`NiagaraFunctionLibrary.SpawnSystemAtLocation` "/Game/Ryddelmyst_Assets/Particles/P_MonsterKillFX.P_MonsterKillFX" _returnvalue)
  (bind _asryddelmyst_game_instance_2 (cast `RyddelmystGameInstance` (`GameplayStatics.GetGameInstance`)))
  (`GameplayStatics.PlaySoundAtLocation` "/Game/Ryddelmyst_Assets/Audio/SFX/bfxr_sounds/Explosion2.Explosion2" _returnvalue (struct) (`RyddelmystGameInstance.SFXVolumeScale` _asryddelmyst_game_instance_2) 1.0 0.0 null null null null)
  (`self.K2_DestroyActor`))

(fn `OnInteract`
  (params (Interactor :type "Actor Object Reference"))
  (returns (ReturnValue :type "Array of InteractCapability Enum"))
  (`KismetSystemLibrary.PrintString` "wooden egg interact")
  (return (`self.InteractCapArray`)))

(fn `UserConstructionScript`)