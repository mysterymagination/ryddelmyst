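; Clockwork Beauty bestiary Blueprint, an interactable that supplies a randomized description paired with a player reaction.
; GenerateDescription picks a random Descriptions entry, maps its index to a reaction (flirty, embarrassed, confused, eldritch, happy as default) and writes both into the returned Descriptor.
; The index-to-reaction mapping is hardcoded, so it depends on the order of Descriptions.
; OnInteract returns InteractCaps, and the event graph holds no active logic.
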(fn `GenerateDescription`
  (returns (ReturnValue :type "Descriptor Structure"))
  (locals (Descriptor :type "Descriptor Structure") (PlayerReaction :type "InteractReactions Enum") (InteractionIndex :type Integer))
  (bind _descriptions (`self.Descriptions`))
  (bind _output_get (set `local.InteractionIndex` (`KismetMathLibrary.RandomIntegerInRange` 0 (- (`KismetArrayLibrary.Array_Length` _descriptions) 1))))
  (switch `int` _output_get
    (:`Default`
      (set `local.PlayerReaction` "HAPPY"))
    (:`0`
      (set `local.PlayerReaction` "FLIRTY"))
    (:`1`
      (set `local.PlayerReaction` "EMBARRASSED"))
    (:`2`
      (set `local.PlayerReaction` "CONFUSED"))
    (:`3`
      (set `local.PlayerReaction` "ELDRITCH")))
  (bind _structout (setmembers `Descriptor` :`StructRef` (`local.Descriptor`) :`LocalizedDescription` (`|GetArrayItem` _descriptions _output_get) :`Reaction` (`local.PlayerReaction`)))
  (return _structout))

(fn `OnInteract`
  (params (Interactor :type "Actor Object Reference"))
  (returns (ReturnValue :type "Array of InteractCapability Enum"))
  (return (`self.InteractCaps`)))

(fn `UserConstructionScript`)