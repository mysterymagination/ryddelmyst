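; AI controller for the Clockwork Beauty enemy that runs its behavior tree on possession and tracks the player as prey.
; A successfully sensed actor tagged Player cancels the forget timer and sets the IsPreySighted and Prey blackboard keys.
; Any other perception update starts a line-of-sight timer, which clears both keys when it expires.
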(event `self.ReceivePossess`
  (params (PossessedPawn :type "Pawn Object Reference"))
  (`self.RunBehaviorTree` "/Game/Ryddelmyst_Assets/Blueprints/AI/Bestiary/ClockworkBeauty/BT_ClockworkBeautyBehavior.BT_ClockworkBeautyBehavior"))

(event `self.AIPerception.OnTargetPerceptionUpdated`
  (params (Actor :type "Actor Object Reference") (Stimulus :type "AIStimulus Structure"))
  (bind _blackboard (`self.Blackboard`))
  (if (and (`self.ActorHasTag` Actor "Player") (`.bSuccessfullySensed` (break `AIStimulus` Stimulus)))
    (`KismetSystemLibrary.K2_ClearAndInvalidateTimerHandle` (`self.EnemyTimer`))
    (`BlackboardComponent.SetValueAsBool` _blackboard (`self.IsPreySighted`) true)
    (`BlackboardComponent.SetValueAsObject` _blackboard (`self.Prey`) Actor)
    (else
      (bind _returnvalue (`KismetSystemLibrary.K2_SetTimerDelegate` (delegate `Start Enemy Timer`) (`self.Line of Sight Timer`)))
      (set `self.EnemyTimer` _returnvalue))))

(event `Start Enemy Timer`
  (bind _blackboard (`self.Blackboard`))
  (`BlackboardComponent.SetValueAsBool` _blackboard (`self.IsPreySighted`) false)
  (`BlackboardComponent.SetValueAsObject` _blackboard (`self.Prey`) null))

(fn `UserConstructionScript`)