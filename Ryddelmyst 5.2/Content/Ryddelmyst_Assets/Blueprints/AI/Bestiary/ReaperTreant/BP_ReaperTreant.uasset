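; Reaper Treant enemy character from the AI bestiary, with separate hit volumes for its body, head, legs and clawed arms.
; On possession it registers both claw capsules with its AI controller as claw "nerves" and hands that controller to its anim instance.
; Every hit volume forwards its component hit events to a shared HitBoxer, keeping hit handling out of this Blueprint.
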(event `self.ReceivePossessed`
  (params (NewController :type "Controller Object Reference"))
  (bind _asbp_reaper_treant_ai (cast `/Game/Ryddelmyst_Assets/Blueprints/AI/Bestiary/ReaperTreant/BP_ReaperTreantAI` (`AIBlueprintHelperLibrary.GetAIController` self)))
  (set `/Game/Ryddelmyst_Assets/Blueprints/AI/Bestiary/ReaperTreant/BP_ReaperTreantAI.RightClawNerve` (`self.ClawCapsuleRightArm`) _asbp_reaper_treant_ai)
  (set `/Game/Ryddelmyst_Assets/Blueprints/AI/Bestiary/ReaperTreant/BP_ReaperTreantAI.LeftClawNerve` (`self.ClawCapsuleLeftArm`) _asbp_reaper_treant_ai)
  (bind _asbp_reaper_treant_anim (cast `/Game/Ryddelmyst_Assets/Animations/BP_ReaperTreantAnim` (`SkeletalMeshComponent.GetAnimInstance` (`self.Mesh`)))
    (:`then`
      (set `/Game/Ryddelmyst_Assets/Animations/BP_ReaperTreantAnim.ReaperTreantAI` _asbp_reaper_treant_ai _asbp_reaper_treant_anim))
    (:`CastFailed`
      (`KismetSystemLibrary.PrintString` "failed to cast anim from treant skel to treantanim"))))

(event `self.BodyBox.OnComponentHit`
  (params (HitComponent :type "PrimitiveComponent Object Reference") (OtherActor :type "Actor Object Reference") (OtherComp :type "PrimitiveComponent Object Reference") (NormalImpulse :type "Vector Structure") (Hit :type "HitResult Structure (by ref)"))
  (`HitBoxerComponent.OnHit` (`self.HitBoxer`) HitComponent OtherActor OtherComp NormalImpulse Hit))

(event `self.HeadBox.OnComponentHit`
  (params (HitComponent :type "PrimitiveComponent Object Reference") (OtherActor :type "Actor Object Reference") (OtherComp :type "PrimitiveComponent Object Reference") (NormalImpulse :type "Vector Structure") (Hit :type "HitResult Structure (by ref)"))
  (`HitBoxerComponent.OnHit` (`self.HitBoxer`) HitComponent OtherActor OtherComp NormalImpulse Hit))

(event `self.ExtremityCapsuleRightLeg.OnComponentHit`
  (params (HitComponent :type "PrimitiveComponent Object Reference") (OtherActor :type "Actor Object Reference") (OtherComp :type "PrimitiveComponent Object Reference") (NormalImpulse :type "Vector Structure") (Hit :type "HitResult Structure (by ref)"))
  (`HitBoxerComponent.OnHit` (`self.HitBoxer`) HitComponent OtherActor OtherComp NormalImpulse Hit))

(event `self.ExtremityCapsuleLeftLeg.OnComponentHit`
  (params (HitComponent :type "PrimitiveComponent Object Reference") (OtherActor :type "Actor Object Reference") (OtherComp :type "PrimitiveComponent Object Reference") (NormalImpulse :type "Vector Structure") (Hit :type "HitResult Structure (by ref)"))
  (`HitBoxerComponent.OnHit` (`self.HitBoxer`) HitComponent OtherActor OtherComp NormalImpulse Hit))

(event `self.ClawCapsuleRightArm.OnComponentHit`
  (params (HitComponent :type "PrimitiveComponent Object Reference") (OtherActor :type "Actor Object Reference") (OtherComp :type "PrimitiveComponent Object Reference") (NormalImpulse :type "Vector Structure") (Hit :type "HitResult Structure (by ref)"))
  (`HitBoxerComponent.OnHit` (`self.HitBoxer`) HitComponent OtherActor OtherComp NormalImpulse Hit))

(event `self.ClawCapsuleLeftArm.OnComponentHit`
  (params (HitComponent :type "PrimitiveComponent Object Reference") (OtherActor :type "Actor Object Reference") (OtherComp :type "PrimitiveComponent Object Reference") (NormalImpulse :type "Vector Structure") (Hit :type "HitResult Structure (by ref)"))
  (`HitBoxerComponent.OnHit` (`self.HitBoxer`) HitComponent OtherActor OtherComp NormalImpulse Hit))

(fn `UserConstructionScript`)