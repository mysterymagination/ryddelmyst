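; AI controller for the Reaper Treant enemy that tracks the player as prey and drives its behavior tree.
; On possess it runs BT_ReaperTreantBehavior, and perception updates from its sniffer component write the prey and sighted flag to the Blackboard.
; Sensing the player cancels the interest timer; any other perception update starts an attention-span timer that clears prey, sighted and within-reach keys when it expires.
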(event `self.ReceivePossess`
  (params (PossessedPawn :type "Pawn Object Reference"))
  (`self.RunBehaviorTree` "/Game/Ryddelmyst_Assets/Blueprints/AI/Bestiary/ReaperTreant/BT_ReaperTreantBehavior.BT_ReaperTreantBehavior"))

(event `self.SnifferOfReaperTreant.OnTargetPerceptionUpdated`
  (params (Actor :type "Actor Object Reference") (Stimulus :type "AIStimulus Structure"))
  (bind (_age _expirationage _strength _stimuluslocation _receiverlocation _tag _bsuccessfullysensed) (break `AIStimulus` Stimulus))
  (bind _blackboard (`self.Blackboard`))
  (`KismetSystemLibrary.PrintString` (`KismetStringLibrary.Concat_StrStr` "sensed: " (`KismetStringLibrary.Conv_BoolToString` _bsuccessfullysensed)))
  (if (and (`self.ActorHasTag` Actor "Player") _bsuccessfullysensed)
    (`KismetSystemLibrary.K2_ClearAndInvalidateTimerHandle` (`self.InterestTimer`))
    (`BlackboardComponent.SetValueAsBool` _blackboard (`self.IsPreySighted`) true)
    (`BlackboardComponent.SetValueAsObject` _blackboard (`self.Prey`) Actor)
    (`KismetSystemLibrary.PrintString` "chasing maya!")
    (else
      (bind _returnvalue (`KismetSystemLibrary.K2_SetTimerDelegate` (delegate `Lose Interest`) (`self.AttentionSpan`)))
      (set `self.InterestTimer` _returnvalue))))

(event `Lose Interest`
  (bind _blackboard (`self.Blackboard`))
  (`BlackboardComponent.SetValueAsBool` _blackboard (`self.IsPreySighted`) false)
  (`BlackboardComponent.SetValueAsObject` _blackboard (`self.Prey`) null)
  (`BlackboardComponent.SetValueAsBool` _blackboard (`self.IsPreyWithinReach`) false)
  (`KismetSystemLibrary.PrintString` "lost track of maya..."))

(fn `UserConstructionScript`)